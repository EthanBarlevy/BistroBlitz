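; BP_Interactable is a base for Bistro Blitz stations that the first-person player can interact with.
; An InteractDistance overlap toggles the InteractPrompt and registers the actor as the character's CurrentInteractable, clearing that reference on exit.
; Interact is an empty function, and the prompt is toggled rather than explicitly shown or hidden.
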(event OnComponentBeginOverlap(InteractDistance)
  (params (OverlappedComponent :type Primitive%20Component%20Object%20Reference) (OtherActor :type Actor%20Object%20Reference) (OtherComp :type Primitive%20Component%20Object%20Reference) (OtherBodyIndex :type Integer) (bFromSweep :type Boolean) (SweepResult :type Hit%20Result%20Structure%20%28by%20ref%29))
  ;[0.03646 0.03646 0.03646] Toggle visibility when entering and exiting the area around the station
  (bind _asbp_first_person_character (Utilities|Casting|CastToBP_FirstPersonCharacter OtherActor))
  (Variables|Default|SetRef_Character _asbp_first_person_character)
  (Rendering|ToggleVisibility (Variables|Default|GetInteractPrompt) false)
  ;[0.03646 0.03646 0.03646] Give the player a reference to self when in range
  (Variables|/Game/FirstPerson/Blueprints/BP_FirstPersonCharacter.BP_FirstPersonCharacter_C|SetCurrentInteractable (Variables|Default|GetRef_Character) self))

(event OnComponentEndOverlap(InteractDistance)
  (params (OverlappedComponent :type Primitive%20Component%20Object%20Reference) (OtherActor :type Actor%20Object%20Reference) (OtherComp :type Primitive%20Component%20Object%20Reference) (OtherBodyIndex :type Integer))
  ;[0.03646 0.03646 0.03646] Toggle visibility when entering and exiting the area around the station
  (Utilities|Casting|CastToBP_FirstPersonCharacter OtherActor)
  (Rendering|ToggleVisibility (Variables|Default|GetInteractPrompt) false)
  ;[0.03646 0.03646 0.03646] Give the player a reference to self when in range
  (Variables|/Game/FirstPerson/Blueprints/BP_FirstPersonCharacter.BP_FirstPersonCharacter_C|SetCurrentInteractable (Variables|Default|GetRef_Character) 0))

(event EventBeginPlay)

(event Collision|EventActorBeginOverlap
  (params (OtherActor :type Actor%20Object%20Reference)))

(event EventTick
  (params (DeltaSeconds :type Float%20%28single-precision%29)))

(fn ConstructionScript)

(fn Interact)