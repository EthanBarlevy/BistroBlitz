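; Game instance for Bistro Blitz that hosts and joins two-player sessions and holds the state of a restaurant shift.
; Ready-up starts the day: a looping timer seats customer groups at random free tables from a randomized spawn budget.
; BP_Fuse events toggle lights and music, and restoring power schedules the next fuse flip.
; It tallies earnings, can randomly spawn messes, and shows the score screen via RemoveFromTable once spawns run out.
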(event Custom|FindTables
  (bind _outactors (Actor|GetAllActorsOfClass "/Game/BistroBlitz/Blueprints/Stations/BP_TableSlot.BP_TableSlot_C"))
  (for _array_element _outactors
    (switch int (Variables|/Game/BistroBlitz/Blueprints/Stations/BP_TableSlot.BP_TableSlot_C|GetTableNumber _array_element)
      (:1
        (Utilities|Array|Add (Variables|Default|GetTable1) _array_element))
      (:2
        (Utilities|Array|Add (Variables|Default|GetTable2) _array_element))
      (:3
        (Utilities|Array|Add (Variables|Default|GetTable3) _array_element))
      (:4
        (Utilities|Array|Add (Variables|Default|GetTable4) _array_element))
      (:5
        (Utilities|Array|Add (Variables|Default|GetTable5) _array_element))))
  (Variables|Default|SetMaxSpawns (Math|Random|RandomIntegerinRange 15 20)))

(event Custom|Host%20Session
  (bind _returnvalue (Game|Player|GetPlayerPawn 0))
  (|AdvancedSession 0 (Game|GetPlayerController 0) 2 0 false true false true true true false false false true false true
    (:OnSuccess
      (Game|OpenLevel(byName) "MainMap" true "Listen")
      (Utilities|FlowControl|Delay 0.2)
      (Transformation|SetActorLocation _returnvalue "446.218644,1855.631669,120.531929" false true)
      (Transformation|SetActorRotation _returnvalue "0.000000,-90.000000,0.000000" true)
      (bind _returnvalue_2 (UserInterface|CreateWidget "/Game/BistroBlitz/UI/UI_Invite.UI_Invite_C" (Game|GetPlayerController 0)))
      (UserInterface|Viewport|AddtoViewport _returnvalue_2 0)
      (Variables|Default|SetNewVar _returnvalue_2)
      (Variables|Default|SetPlayersReady 0)
      (CallFunction|FindTables))))

(event Custom|TurnPowerOn
  (CallFunction|EnableLights)
  (Default|Start (Variables|Default|GetMusic))
  (Variables|Default|SetPowerState true)
  (CallFunction|TurnPowerOff))

(event Custom|Turn%20Off
  (CallFunction|TurnItOff))

(event Custom|TurnPowerOff
  (Utilities|FlowControl|Delay (Math|Random|RandomFloatinRange 1e+01 1e+01))
  (bind _returnvalue (Actor|GetActorOfClass "/Game/BistroBlitz/Blueprints/Stations/BP_Fuse.BP_Fuse_C"))
  (Default|Flip _returnvalue))

(event Custom|Enable%20Lights
  (for _array_element (Variables|Default|GetLights)
    (Default|ChangeStateMulti _array_element)))

(event Custom|TurnItOff
  (for _array_element (Variables|Default|GetLights)
    (Default|ChangeStateMulti _array_element))
  (Variables|Default|SetPowerState false)
  (Audio|PlaySound2D "/Game/BistroBlitz/Audio/Poweroff_Cue.Poweroff_Cue" 1.0 1.0 0.0 0 0)
  (Default|Stop (Variables|Default|GetMusic)))

(event Custom|Unready
  (Math|Integer|DecrementInt (Variables|Default|GetPlayersReady)))

(event Custom|StartDay
  (Utilities|Time|SetTimerbyEvent (delegate Custom|CustomEvent) 8e+01 true)
  (CallFunction|CustomEvent)
  (CallFunction|FindLights)
  (bind _returnvalue (Actor|GetActorOfClass "/Game/BistroBlitz/Blueprints/Stations/BP_Fuse.BP_Fuse_C"))
  (EventDispatchers|BindEventtoPoweron _returnvalue (delegate Custom|TurnPowerOn))
  (bind _returnvalue_2 (Game|SpawnActorfromClass "/Game/BistroBlitz/Blueprints/BP_Music.BP_Music_C" (Math|Transform|MakeTransform "-427.339257,1580.299162,15.143947") "Undefined" "MultiplyWithRoot" 0 0))
  (Variables|Default|SetMusic _returnvalue_2)
  (EventDispatchers|BindEventtoTurnOff _returnvalue (delegate Custom|Turn%20Off))
  (Variables|Default|SetIsGameStarted true)
  (Default|CallGameStarted))

(event Custom|CustomEvent
  (if (< (Variables|Default|GetTablesFilled) 3)
    (while (Variables|Default|GetFreeTable)
      (Variables|Default|SetTableNumber (+ (Math|Random|RandomIntegerinRange 0 4) 1))
      (Variables|Default|SetFreeTable (not (== (Utilities|Array|Get(acopy) (Variables|Default|GetNumberAtTable) (- (Variables|Default|GetTableNumber) 1)) 0))))
    (switch int (Variables|Default|GetTableNumber)
      (:1
        (for _index (range 0 (Math|Random|RandomIntegerinRange 2 3))
          (if (> (Variables|Default|GetMaxSpawns) 0)
            (bind _returnvalue (Game|SpawnActorfromClass "/Game/BistroBlitz/Blueprints/AI/BP_BistroBlitzCustomer.BP_BistroBlitzCustomer_C" (Math|Transform|MakeTransform "-1220.000000,1150.000000,104.531949" "0.000000,-90.000000,0.000000") "Undefined" "MultiplyWithRoot" 0 0))
            (Utilities|Array|Add (Variables|Default|GetCustomers) _returnvalue)
            (bind _result (Math|Integer|DecrementInt (Variables|Default|GetMaxSpawns))
              (:%20%20
                (Variables|/Game/BistroBlitz/Blueprints/AI/BP_BistroBlitzCustomer.BP_BistroBlitzCustomer_C|SetID _returnvalue _result)))))
        (Utilities|FlowControl|Delay 1.0)
        (for (_array_element _array_index) (Variables|Default|GetCustomers)
          (bind _returnvalue_2 (Actor|GetActorOfClass "/Game/BistroBlitz/Blueprints/AI/BP_CustomerExit.BP_CustomerExit_C"))
          (Variables|/Game/BistroBlitz/Blueprints/AI/BP_BistroBlitzCustomer.BP_BistroBlitzCustomer_C|SetChairID _array_element (Variables|/Game/BistroBlitz/Blueprints/Stations/BP_TableSlot.BP_TableSlot_C|GetSeatNumber (Utilities|Array|Get(acopy) (Variables|Default|GetTable1) _array_index)))
          (Variables|/Game/BistroBlitz/Blueprints/Stations/BP_TableSlot.BP_TableSlot_C|SetCustomerID (Utilities|Array|Get(acopy) (Variables|Default|GetTable1) _array_index) (Variables|/Game/BistroBlitz/Blueprints/AI/BP_BistroBlitzCustomer.BP_BistroBlitzCustomer_C|GetID _array_element))
          (Default|SetTableSlot _array_element (Variables|/Game/BistroBlitz/Blueprints/Stations/BP_TableSlot.BP_TableSlot_C|GetSeatNumber (Utilities|Array|Get(acopy) (Variables|Default|GetTable1) _array_index)) _returnvalue_2)
          (Variables|/Game/BistroBlitz/Blueprints/AI/BP_BistroBlitzCustomer.BP_BistroBlitzCustomer_C|SetCurrentInteractable _array_element (Utilities|Array|Get(acopy) (Variables|Default|GetTable1) _array_index))
          (Variables|/Game/BistroBlitz/Blueprints/Stations/BP_TableSlot.BP_TableSlot_C|SetCustomer (Utilities|Array|Get(acopy) (Variables|Default|GetTable1) _array_index) _array_element)
          (Math|Integer|IncrementInt (Utilities|Array|Get(acopy) (Variables|Default|GetNumberAtTable))
            (:%20%20
              (Variables|Default|SetFreeTable true))))
        (Utilities|Array|Clear (Variables|Default|GetCustomers))
        (Math|Integer|IncrementInt (Variables|Default|GetTablesFilled)))
      (:2
        (for _index_2 (range 0 (Math|Random|RandomIntegerinRange 0 1))
          (if (> (Variables|Default|GetMaxSpawns) 0)
            (bind _returnvalue_3 (Game|SpawnActorfromClass "/Game/BistroBlitz/Blueprints/AI/BP_BistroBlitzCustomer.BP_BistroBlitzCustomer_C" (Math|Transform|MakeTransform "-1220.000000,1150.000000,104.531949" "0.000000,-90.000000,0.000000") "Undefined" "MultiplyWithRoot" 0 0))
            (Utilities|Array|Add (Variables|Default|GetCustomers) _returnvalue_3)
            (bind _result_2 (Math|Integer|DecrementInt (Variables|Default|GetMaxSpawns))
              (:%20%20
                (Variables|/Game/BistroBlitz/Blueprints/AI/BP_BistroBlitzCustomer.BP_BistroBlitzCustomer_C|SetID _returnvalue_3 _result_2)))))
        (Utilities|FlowControl|Delay 1.0)
        (for (_array_element_2 _array_index_2) (Variables|Default|GetCustomers)
          (bind _returnvalue_4 (Actor|GetActorOfClass "/Game/BistroBlitz/Blueprints/AI/BP_CustomerExit.BP_CustomerExit_C"))
          (Variables|/Game/BistroBlitz/Blueprints/AI/BP_BistroBlitzCustomer.BP_BistroBlitzCustomer_C|SetChairID _array_element_2 (Variables|/Game/BistroBlitz/Blueprints/Stations/BP_TableSlot.BP_TableSlot_C|GetSeatNumber (Utilities|Array|Get(acopy) (Variables|Default|GetTable2) _array_index_2)))
          (Variables|/Game/BistroBlitz/Blueprints/Stations/BP_TableSlot.BP_TableSlot_C|SetCustomerID (Utilities|Array|Get(acopy) (Variables|Default|GetTable2) _array_index_2) (Variables|/Game/BistroBlitz/Blueprints/AI/BP_BistroBlitzCustomer.BP_BistroBlitzCustomer_C|GetID _array_element_2))
          (Default|SetTableSlot _array_element_2 (Variables|/Game/BistroBlitz/Blueprints/Stations/BP_TableSlot.BP_TableSlot_C|GetSeatNumber (Utilities|Array|Get(acopy) (Variables|Default|GetTable2) _array_index_2)) _returnvalue_4)
          (Variables|/Game/BistroBlitz/Blueprints/AI/BP_BistroBlitzCustomer.BP_BistroBlitzCustomer_C|SetCurrentInteractable _array_element_2 (Utilities|Array|Get(acopy) (Variables|Default|GetTable2) _array_index_2))
          (Variables|/Game/BistroBlitz/Blueprints/Stations/BP_TableSlot.BP_TableSlot_C|SetCustomer (Utilities|Array|Get(acopy) (Variables|Default|GetTable2) _array_index_2) _array_element_2)
          (Math|Integer|IncrementInt (Utilities|Array|Get(acopy) (Variables|Default|GetNumberAtTable) 1)
            (:%20%20
              (Variables|Default|SetFreeTable true))))
        (Utilities|Array|Clear (Variables|Default|GetCustomers))
        (Math|Integer|IncrementInt (Variables|Default|GetTablesFilled)))
      (:3
        (for _index_3 (range 0 (Math|Random|RandomIntegerinRange 0 1))
          (if (> (Variables|Default|GetMaxSpawns) 0)
            (bind _returnvalue_5 (Game|SpawnActorfromClass "/Game/BistroBlitz/Blueprints/AI/BP_BistroBlitzCustomer.BP_BistroBlitzCustomer_C" (Math|Transform|MakeTransform "-1220.000000,1150.000000,104.531949" "0.000000,-90.000000,0.000000") "Undefined" "MultiplyWithRoot" 0 0))
            (Utilities|Array|Add (Variables|Default|GetCustomers) _returnvalue_5)
            (bind _result_3 (Math|Integer|DecrementInt (Variables|Default|GetMaxSpawns))
              (:%20%20
                (Variables|/Game/BistroBlitz/Blueprints/AI/BP_BistroBlitzCustomer.BP_BistroBlitzCustomer_C|SetID _returnvalue_5 _result_3)))))
        (Utilities|FlowControl|Delay 1.0)
        (for (_array_element_3 _array_index_3) (Variables|Default|GetCustomers)
          (bind _returnvalue_6 (Actor|GetActorOfClass "/Game/BistroBlitz/Blueprints/AI/BP_CustomerExit.BP_CustomerExit_C"))
          (Variables|/Game/BistroBlitz/Blueprints/AI/BP_BistroBlitzCustomer.BP_BistroBlitzCustomer_C|SetChairID _array_element_3 (Variables|/Game/BistroBlitz/Blueprints/Stations/BP_TableSlot.BP_TableSlot_C|GetSeatNumber (Utilities|Array|Get(acopy) (Variables|Default|GetTable3) _array_index_3)))
          (Variables|/Game/BistroBlitz/Blueprints/Stations/BP_TableSlot.BP_TableSlot_C|SetCustomerID (Utilities|Array|Get(acopy) (Variables|Default|GetTable3) _array_index_3) (Variables|/Game/BistroBlitz/Blueprints/AI/BP_BistroBlitzCustomer.BP_BistroBlitzCustomer_C|GetID _array_element_3))
          (Default|SetTableSlot _array_element_3 (Variables|/Game/BistroBlitz/Blueprints/Stations/BP_TableSlot.BP_TableSlot_C|GetSeatNumber (Utilities|Array|Get(acopy) (Variables|Default|GetTable3) _array_index_3)) _returnvalue_6)
          (Variables|/Game/BistroBlitz/Blueprints/AI/BP_BistroBlitzCustomer.BP_BistroBlitzCustomer_C|SetCurrentInteractable _array_element_3 (Utilities|Array|Get(acopy) (Variables|Default|GetTable3) _array_index_3))
          (Variables|/Game/BistroBlitz/Blueprints/Stations/BP_TableSlot.BP_TableSlot_C|SetCustomer (Utilities|Array|Get(acopy) (Variables|Default|GetTable3) _array_index_3) _array_element_3)
          (Math|Integer|IncrementInt (Utilities|Array|Get(acopy) (Variables|Default|GetNumberAtTable) 2)
            (:%20%20
              (Variables|Default|SetFreeTable true))))
        (Utilities|Array|Clear (Variables|Default|GetCustomers))
        (Math|Integer|IncrementInt (Variables|Default|GetTablesFilled)))
      (:4
        (for _index_4 (range 0 (Math|Random|RandomIntegerinRange 2 3))
          (if (> (Variables|Default|GetMaxSpawns) 0)
            (bind _returnvalue_7 (Game|SpawnActorfromClass "/Game/BistroBlitz/Blueprints/AI/BP_BistroBlitzCustomer.BP_BistroBlitzCustomer_C" (Math|Transform|MakeTransform "-1220.000000,1150.000000,104.531949" "0.000000,-90.000000,0.000000") "Undefined" "MultiplyWithRoot" 0 0))
            (Utilities|Array|Add (Variables|Default|GetCustomers) _returnvalue_7)
            (bind _result_4 (Math|Integer|DecrementInt (Variables|Default|GetMaxSpawns))
              (:%20%20
                (Variables|/Game/BistroBlitz/Blueprints/AI/BP_BistroBlitzCustomer.BP_BistroBlitzCustomer_C|SetID _returnvalue_7 _result_4)))))
        (Utilities|FlowControl|Delay 1.0)
        (for (_array_element_4 _array_index_4) (Variables|Default|GetCustomers)
          (bind _returnvalue_8 (Actor|GetActorOfClass "/Game/BistroBlitz/Blueprints/AI/BP_CustomerExit.BP_CustomerExit_C"))
          (Variables|/Game/BistroBlitz/Blueprints/AI/BP_BistroBlitzCustomer.BP_BistroBlitzCustomer_C|SetChairID _array_element_4 (Variables|/Game/BistroBlitz/Blueprints/Stations/BP_TableSlot.BP_TableSlot_C|GetSeatNumber (Utilities|Array|Get(acopy) (Variables|Default|GetTable4) _array_index_4)))
          (Variables|/Game/BistroBlitz/Blueprints/Stations/BP_TableSlot.BP_TableSlot_C|SetCustomerID (Utilities|Array|Get(acopy) (Variables|Default|GetTable4) _array_index_4) (Variables|/Game/BistroBlitz/Blueprints/AI/BP_BistroBlitzCustomer.BP_BistroBlitzCustomer_C|GetID _array_element_4))
          (Default|SetTableSlot _array_element_4 (Variables|/Game/BistroBlitz/Blueprints/Stations/BP_TableSlot.BP_TableSlot_C|GetSeatNumber (Utilities|Array|Get(acopy) (Variables|Default|GetTable4) _array_index_4)) _returnvalue_8)
          (Variables|/Game/BistroBlitz/Blueprints/AI/BP_BistroBlitzCustomer.BP_BistroBlitzCustomer_C|SetCurrentInteractable _array_element_4 (Utilities|Array|Get(acopy) (Variables|Default|GetTable4) _array_index_4))
          (Variables|/Game/BistroBlitz/Blueprints/Stations/BP_TableSlot.BP_TableSlot_C|SetCustomer (Utilities|Array|Get(acopy) (Variables|Default|GetTable4) _array_index_4) _array_element_4)
          (Math|Integer|IncrementInt (Utilities|Array|Get(acopy) (Variables|Default|GetNumberAtTable) 3)
            (:%20%20
              (Variables|Default|SetFreeTable true))))
        (Utilities|Array|Clear (Variables|Default|GetCustomers))
        (Math|Integer|IncrementInt (Variables|Default|GetTablesFilled)))
      (:5
        (for _index_5 (range 0 (Math|Random|RandomIntegerinRange 0 1))
          (if (> (Variables|Default|GetMaxSpawns) 0)
            (bind _returnvalue_9 (Game|SpawnActorfromClass "/Game/BistroBlitz/Blueprints/AI/BP_BistroBlitzCustomer.BP_BistroBlitzCustomer_C" (Math|Transform|MakeTransform "-1220.000000,1150.000000,104.531949" "0.000000,-90.000000,0.000000") "Undefined" "MultiplyWithRoot" 0 0))
            (Utilities|Array|Add (Variables|Default|GetCustomers) _returnvalue_9)
            (bind _result_5 (Math|Integer|DecrementInt (Variables|Default|GetMaxSpawns))
              (:%20%20
                (Variables|/Game/BistroBlitz/Blueprints/AI/BP_BistroBlitzCustomer.BP_BistroBlitzCustomer_C|SetID _returnvalue_9 _result_5)))))
        (Utilities|FlowControl|Delay 1.0)
        (for (_array_element_5 _array_index_5) (Variables|Default|GetCustomers)
          (bind _returnvalue_10 (Actor|GetActorOfClass "/Game/BistroBlitz/Blueprints/AI/BP_CustomerExit.BP_CustomerExit_C"))
          (Variables|/Game/BistroBlitz/Blueprints/AI/BP_BistroBlitzCustomer.BP_BistroBlitzCustomer_C|SetChairID _array_element_5 (Variables|/Game/BistroBlitz/Blueprints/Stations/BP_TableSlot.BP_TableSlot_C|GetSeatNumber (Utilities|Array|Get(acopy) (Variables|Default|GetTable5) _array_index_5)))
          (Variables|/Game/BistroBlitz/Blueprints/Stations/BP_TableSlot.BP_TableSlot_C|SetCustomerID (Utilities|Array|Get(acopy) (Variables|Default|GetTable5) _array_index_5) (Variables|/Game/BistroBlitz/Blueprints/AI/BP_BistroBlitzCustomer.BP_BistroBlitzCustomer_C|GetID _array_element_5))
          (Default|SetTableSlot _array_element_5 (Variables|/Game/BistroBlitz/Blueprints/Stations/BP_TableSlot.BP_TableSlot_C|GetSeatNumber (Utilities|Array|Get(acopy) (Variables|Default|GetTable5) _array_index_5)) _returnvalue_10)
          (Variables|/Game/BistroBlitz/Blueprints/Stations/BP_TableSlot.BP_TableSlot_C|SetCustomer (Utilities|Array|Get(acopy) (Variables|Default|GetTable5) _array_index_5) _array_element_5)
          (Variables|/Game/BistroBlitz/Blueprints/AI/BP_BistroBlitzCustomer.BP_BistroBlitzCustomer_C|SetCurrentInteractable _array_element_5 (Utilities|Array|Get(acopy) (Variables|Default|GetTable5) _array_index_5))
          (Math|Integer|IncrementInt (Utilities|Array|Get(acopy) (Variables|Default|GetNumberAtTable) 4)
            (:%20%20
              (Variables|Default|SetFreeTable true))))
        (Utilities|Array|Clear (Variables|Default|GetCustomers))
        (Math|Integer|IncrementInt (Variables|Default|GetTablesFilled))))))

(event Custom|ResetEverything
  (Utilities|Array|Clear (Variables|Default|GetTable1))
  (Variables|Default|SetIndex 0)
  (Variables|Default|SetSpawned 0)
  (Utilities|Array|Clear (Variables|Default|GetTable2))
  (Utilities|Array|Clear (Variables|Default|GetTable3))
  (Utilities|Array|Clear (Variables|Default|GetTable4))
  (Utilities|Array|Clear (Variables|Default|GetTable5))
  (Utilities|Array|Clear (Variables|Default|GetCustomers))
  (Utilities|Array|Clear (Variables|Default|GetLights))
  (Variables|Default|SetTotalMoneyEarned 0.0)
  (Variables|Default|SetIsGameStarted false)
  (Variables|Default|SetPlayersReady 0)
  (Variables|Default|SetPowerState true))

(event Custom|remove
  (bind _newvar (Variables|Default|GetNewVar))
  (Utilities|IsValid _newvar
    (:Is%20Valid
      (Widget|RemovefromParent _newvar))))

(event Custom|Ready
  (bind _result (Math|Integer|IncrementInt (Variables|Default|GetPlayersReady))
    (:%20%20
      (if (== _result 1)
        (CallFunction|StartDay)
        (else
          (CallFunction|FindTables))))))

(event Custom|end
  (bind _returnvalue (Game|GetPlayerController 0))
  (bind _returnvalue_2 (UserInterface|CreateWidget "/Game/BistroBlitz/UI/UI_Score.UI_Score_C" _returnvalue))
  (bind _asui_score (Utilities|Casting|CastToUI_Score _returnvalue_2))
  (Default|Setmoney _asui_score (Variables|Default|GetTotalMoneyEarned))
  (UserInterface|Viewport|AddtoViewport _returnvalue_2 0)
  (Input|SetInputModeUIOnly _returnvalue _returnvalue_2 "DoNotLock" false)
  (Variables|/Script/Engine.PlayerController|SetbShowMouseCursor _returnvalue true))

(event Custom|TrySpawnMess
  (if (< (Math|Random|RandomFloat) 0.005)
    (bind _returnvalue (Actor|GetActorOfClass "/Game/BistroBlitz/Blueprints/BP_MessSpawner.BP_MessSpawner_C"))
    (Default|SpawnMessServer _returnvalue)))

(event Custom|FindLights
  (bind _outactors (Actor|GetAllActorsOfClass "/Game/BistroBlitz/Blueprints/BP_LightFixture.BP_LightFixture_C"))
  (Variables|Default|SetLights _outactors))

(event EventOnSessionInviteAccepted
  (params (LocalPlayerNum :type Integer) (PersonInvited :type BP%20Unique%20Net%20Id%20Structure) (SessionToJoin :type Blueprint%20Session%20Result%20Structure%20%28by%20ref%29))
  (bind _returnvalue (Game|Player|GetPlayerPawn 0))
  (|JoinSession (Game|GetPlayerController 0) SessionToJoin
    (:OnSuccess
      (Transformation|SetActorLocation _returnvalue "-110.365218,1363.599189,120.531929" false true)
      (Transformation|SetActorRotation _returnvalue "0.000000,90.000000,0.000000" true)
      (Utilities|FlowControl|Delay 5.0))))

(event EventInit
  (Utilities|FlowControl|Delay 1.0)
  (CallFunction|FindTables))

(fn RemovefromTable
  (params (TableNumber :type Integer))
  (Math|Integer|DecrementInt (Utilities|Array|Get(acopy) (Variables|Default|GetNumberAtTable) (- TableNumber 1))
    (:%20%20
      (Math|Integer|DecrementInt (Variables|Default|GetTablesFilled)
        (:%20%20
          (if (not (> (Variables|Default|GetMaxSpawns) 0))
            (CallFunction|End)))))))

(fn AddScore
  (params (PercentClose :type Float%20%28double-precision%29) (Price :type Float%20%28double-precision%29))
  (Variables|Default|SetTotalMoneyEarned (+ (Variables|Default|GetTotalMoneyEarned) (* Price PercentClose)))
  (Default|CallMoneyChanged))