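; First-person player character for multiplayer Bistro Blitz that interacts with objects and carries one holdable, such as an order.
; A per-tick sphere trace, gated by authority and a Host flag, finds interactables and drives the controller's prompt.
; E passes the held item to the interactable.
; Tick refreshes the held mesh and order widget and re-resolves the holdable by class and ID, with BP_Nothing representing empty hands.
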(event Custom|setid
  (CallFunction|SetidMulti))

(event Custom|set%20holding%20server
  (CallFunction|SetHoldingMulti))

(event Custom|setid%20multi
  (Variables|Default|SetID 1))

(event Custom|SetOrder%20Server
  (params (ActorClass :type Actor%20Class%20Reference) (id :type Integer))
  (bind _outactors (Actor|GetAllActorsOfClass ActorClass))
  (for _array_element _outactors
    (bind _asbp_order (Utilities|Casting|CastToBP_Order _array_element)
      (:then
        (if (== (Variables|/Game/BistroBlitz/Blueprints/Holdables/BP_Holdable.BP_Holdable_C|GetID _asbp_order) id)
          (UserInterface|SetWidget (Variables|Default|GetOrder) (UserInterface|GetWidget (Variables|/Game/BistroBlitz/Blueprints/Holdables/BP_Order.BP_Order_C|GetWidget _asbp_order)))))
      (:CastFailed
        (bind _asbp_nothing (Utilities|Casting|CastToBP_Nothing _array_element))
        (UserInterface|SetWidget (Variables|Default|GetOrder) (UserInterface|GetWidget (Variables|/Game/BistroBlitz/Blueprints/Holdables/BP_Nothing.BP_Nothing_C|GetWidget _asbp_nothing)))))))

(event Custom|set%20holding%20multi
  (Variables|Default|SetHolding false))

(event Custom|CustomEvent
  (Variables|Default|SetgameStarted (Variables|/Game/BistroBlitz/Blueprints/GI_ServerInfo.GI_ServerInfo_C|GetIsGameStarted (stale EventBeginPlay _asgi_server_info_2))))

(event Custom|SetHoldable%20Server
  (params (Holdable :type BP%20Holdable%20Object%20Reference) (HoldableClass :type BP%20Holdable%20Class%20Reference) (Index :type Integer) (Nothing :type Boolean))
  (CallFunction|SetHolding Holdable HoldableClass Index Nothing))

(event Custom|set%20id
  (bind _outactors (Actor|GetAllActorsOfClass "BP_BistroBlitzCharacter_C"))
  (bind _output_get (Variables|Default|SetPersonalID (Utilities|Array|Length _outactors)))
  (bind _result (Math|Integer|DecrementInt _output_get)
    (:%20%20
      (if (> _result 0)
        (Variables|Default|Sethost false)
        (else
          (Variables|Default|Sethost true))))))

(event EventBeginPlay
  ;[0.03646 0.03646 0.03646] Owner visiblility things
  (Actor|SetOwner (Game|GetPlayerController 0))
  (Class|PrimitiveComponent|SetOwnerNoSee (Variables|Character|GetMesh) true)
  (Rendering|SetOnlyOwnerSee (Variables|Default|GetHoldingFirstPerson) true :!class /Script/Engine.PrimitiveComponent)
  (Rendering|SetOnlyOwnerSee (Variables|Default|GetOrder) true :!class /Script/Engine.PrimitiveComponent)
  (bind _asgi_server_info (Utilities|Casting|CastToGI_ServerInfo (Game|GetGameInstance)))
  (Variables|Default|SetID (Variables|/Game/BistroBlitz/Blueprints/GI_ServerInfo.GI_ServerInfo_C|GetIndex _asgi_server_info))
  (bind _returnvalue (Actor|GetActorOfClass "/Game/BistroBlitz/Blueprints/Holdables/BP_Nothing.BP_Nothing_C"))
  (Variables|Default|SetHoldable _returnvalue)
  (CallFunction|SetId)
  (bind _asgi_server_info_2 (Utilities|Casting|CastToGI_ServerInfo (Game|GetGameInstance)))
  (EventDispatchers|BindEventtoGameStarted _asgi_server_info_2 (delegate Custom|CustomEvent)))

(event EventTick
  (params (DeltaSeconds :type Float%20%28single-precision%29))
  (bind _firstpersoncameracomponent (Variables|Default|GetFirstPersonCameraComponent))
  (bind _host (Variables|Default|Gethost))
  (bind _returnvalue (Transformation|GetWorldLocation _firstpersoncameracomponent))
  ;[0.03646 0.03646 0.03646] idk for some reason they dont update properly
  (Utilities|FlowControl|Sequence
    (:then_0
      (Utilities|IsValid (Variables|Default|GetHoldable)
        (:Is%20Valid
          (CallFunction|UpdateHolding)
          (bind _asbp_order (Utilities|Casting|CastToBP_Order (Variables|Default|GetHoldable))
            (:then
              (CallFunction|SetOrderServer "/Game/BistroBlitz/Blueprints/Holdables/BP_Order.BP_Order_C" (Variables|/Game/BistroBlitz/Blueprints/Holdables/BP_Holdable.BP_Holdable_C|GetID _asbp_order)))
            (:CastFailed
              (Utilities|Casting|CastToBP_Nothing (Variables|Default|GetHoldable))
              (CallFunction|SetOrderServer "/Game/BistroBlitz/Blueprints/Holdables/BP_Nothing.BP_Nothing_C"))))))
    (:then_1
      (Networking|SwitchHasAuthority
        (:Authority
          (if _host
            ;[0.03646 0.03646 0.03646] Find interactables
            (bind _outhits (Collision|MultiSphereTraceForObjects _returnvalue (+ _returnvalue (* (Math|Vector|GetForwardVector (Variables|Default|GetArrow1)) (Variables|Default|GetInteractionDistance))) 1.0 (Utilities|Array|MakeArray "ObjectTypeQuery2" "ObjectTypeQuery1") false 0 "None" :!label _label))
            (if (> (Utilities|Array|Length _outhits) 0)
              (bind _array_element (Utilities|Array|ForEachLoopwithBreak _outhits :!label _label_2)
                (:LoopBody
                  (bind _asbp_interactable (Utilities|Casting|CastToBP_Interactable (.HitActor (Collision|BreakHitResult _array_element)))
                    (:then
                      (bind _output_get (Variables|Default|SetCurrentInteractable _asbp_interactable))
                      (bind (_flavortext _singleinteraction _radialamount _just_ft) (Default|GetInteractionInformation _output_get (Variables|Default|GetHoldable)))
                      (bind _aspc_bistro_blitz (Utilities|Casting|CastToPC_BistroBlitz (Game|GetPlayerController 0)))
                      (Default|ShowInteraction _aspc_bistro_blitz _flavortext _singleinteraction _radialamount _just_ft (Networking|IsServer))
                      (goto _label_2 Break))
                    (:CastFailed
                      (Utilities|Casting|CastToBlockingVolume (.HitActor (Collision|BreakHitResult _array_element))
                        (:CastFailed
                          (bind _aspc_bistro_blitz_2 (Utilities|Casting|CastToPC_BistroBlitz (Game|GetPlayerController 0)))
                          (Default|SetVisibilty _aspc_bistro_blitz_2 "Hidden" false (Networking|IsServer))
                          (goto _label_2 Break)))))))
              (else
                (bind _aspc_bistro_blitz_3 (Utilities|Casting|CastToPC_BistroBlitz (Game|GetPlayerController 0)))
                (Default|SetVisibilty _aspc_bistro_blitz_3 "Hidden" false (Networking|IsServer))))))
        (:Remote
          (if (not _host)
            (goto _label)))))
    (:then_2
      (bind _outactors (Actor|GetAllActorsOfClass (Variables|Default|GetHoldable%20Class)))
      (for _array_element_2 _outactors
        (if (== (Variables|/Game/BistroBlitz/Blueprints/Holdables/BP_Holdable.BP_Holdable_C|GetID _array_element_2) (Variables|Default|GetID))
          (Variables|Default|SetHoldable _array_element_2))))))

(event Input|KeyboardEvents|DebugKeyP
  (params (Key :type Key%20Structure :default "None") (ActionValue :type Input%20Action%20Value%20Structure))
  (:Pressed
    (Development|PrintString (Utilities|String|ToString(Boolean) (Variables|Default|GetHolding)) true true "(R=1.000000,G=0.686723,B=0.000000,A=1.000000)" 27.0)))

(event Input|KeyboardEvents|E
  (params (Key :type Key%20Structure :default "None"))
  (bind _self self)
  (bind _holdable (Variables|Default|GetHoldable))
  (bind _returnvalue (Utilities|GetClass _holdable))
  (bind _id (Variables|/Game/BistroBlitz/Blueprints/Holdables/BP_Holdable.BP_Holdable_C|GetID _holdable))
  ;[0.03646 0.03646 0.03646] Interact with interactable
  (:Pressed
    (Development|PrintString (Utilities|String|ToString(Name) (Variables|/Game/BistroBlitz/Blueprints/Holdables/BP_Holdable.BP_Holdable_C|GetName (Variables|Default|GetHoldable))) true true "(R=1.000000,G=0.000000,B=0.370127,A=1.000000)")
    (Utilities|IsValid (Variables|Default|GetCurrentInteractable)
      (:Is%20Valid
        (Default|Interacted (Variables|Default|GetCurrentInteractable) _holdable _self _id _returnvalue)
        (Utilities|IsValid (Variables|Default|GetCurrentInteractable)
          (:Is%20Valid
            (Default|InteractNoRep (Variables|Default|GetCurrentInteractable) _self _holdable _id _returnvalue)
            (Variables|Default|SetCurrentInteractable 0)
            (Development|PrintString (Utilities|String|ToString(Name) (Variables|/Game/BistroBlitz/Blueprints/Holdables/BP_Holdable.BP_Holdable_C|GetName (Variables|Default|GetHoldable))) true true "(R=1.000000,G=0.637823,B=0.262179,A=1.000000)")))))))

(fn ConstructionScript)

(fn UpdateHolding
  (Components|StaticMesh|SetStaticMesh (Variables|Default|GetHoldingFirstPerson) (Variables|/Script/Engine.StaticMeshComponent|GetStaticMesh (Variables|/Game/BistroBlitz/Blueprints/Holdables/BP_Holdable.BP_Holdable_C|GetStaticMesh (Variables|Default|GetHoldable)))))

(fn SetHolding
  (params (Holdable :type BP%20Holdable%20Object%20Reference) (HoldableClass :type BP%20Holdable%20Class%20Reference) (Index :type Integer) (Nothing :type Boolean))
  (if Nothing
    (Variables|Default|SetHoldable%20Class "/Game/BistroBlitz/Blueprints/Holdables/BP_Nothing.BP_Nothing_C")
    (bind _returnvalue (Actor|GetActorOfClass "/Game/BistroBlitz/Blueprints/Holdables/BP_Nothing.BP_Nothing_C"))
    (Variables|Default|SetHoldable _returnvalue)
    (Variables|Default|SetHolding false)
    (CallFunction|SetOrderServer "/Game/BistroBlitz/Blueprints/Holdables/BP_Nothing.BP_Nothing_C")
    (CallFunction|SetHoldingServer)
    (else
      (bind _output_get (Variables|Default|SetHoldable%20Class HoldableClass))
      (Variables|Default|SetID Index)
      (bind _outactors (Actor|GetAllActorsOfClass _output_get))
      (bind _array_element (Utilities|Array|ForEachLoopwithBreak _outactors :!label _label)
        (:LoopBody
          (if (== (Variables|/Game/BistroBlitz/Blueprints/Holdables/BP_Holdable.BP_Holdable_C|GetID _array_element) Index)
            (Variables|Default|SetHoldable _array_element)
            (goto _label Break)))
        (:Completed
          (bind _isnothing (Default|GetObjectInformation (Variables|Default|GetHoldable)))
          (Variables|Default|SetHolding (not _isnothing))
          (bind _asbp_order (Utilities|Casting|CastToBP_Order (Variables|Default|GetHoldable))
            (:then
              (CallFunction|SetOrderServer "/Game/BistroBlitz/Blueprints/Holdables/BP_Order.BP_Order_C" (Variables|/Game/BistroBlitz/Blueprints/Holdables/BP_Holdable.BP_Holdable_C|GetID _asbp_order)))
            (:CastFailed
              (Utilities|Casting|CastToBP_Nothing (Variables|Default|GetHoldable))
              (CallFunction|SetOrderServer "/Game/BistroBlitz/Blueprints/Holdables/BP_Nothing.BP_Nothing_C"))))))))