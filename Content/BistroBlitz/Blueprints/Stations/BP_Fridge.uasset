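; BP_Fridge is an interactable kitchen station that opens a fridge menu for the player in Bistro Blitz.
; InteractNoRep creates the UI_Fridge widget for the character's local player controller, reusing it if still valid, and adds it to the viewport.
; It then switches that controller to UI-only input focused on the widget and shows the mouse cursor.
; The replicated Interact only calls its parent.
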(event EventBeginPlay
  (|CallParentFunction) ; This node is disabled and will not be called.\nDrag off pins to build functionality.
)

(event Collision|EventActorBeginOverlap
  (params (OtherActor :type Actor%20Object%20Reference))
  (|CallParentFunction OtherActor) ; This node is disabled and will not be called.\nDrag off pins to build functionality.
)

(event EventTick
  (params (DeltaSeconds :type Float%20%28single-precision%29))
  (|CallParentFunction DeltaSeconds) ; This node is disabled and will not be called.\nDrag off pins to build functionality.
)

(fn ConstructionScript
  (|CallParentFunction))

(fn Interact
  (params (CurrentHoldable :type BP%20Holdable%20Object%20Reference) (CurrentPlayer :type BP%20Bistro%20Blitz%20Character%20Object%20Reference) (ItemIndex :type Integer) (HoldableType :type BP%20Holdable%20Class%20Reference))
  (|CallParentFunction 0 0 0 0))

(fn InteractNoRep
  (params (character :type BP%20Bistro%20Blitz%20Character%20Object%20Reference) (holdable :type BP%20Holdable%20Object%20Reference) (ItemIndex :type Integer) (HoldableType :type BP%20Holdable%20Class%20Reference))
  (bind _returnvalue (Pawn|GetLocalViewingPlayerController character))
  (|CallParentFunction 0 0 0 0)
  (Utilities|IsValid (stale _returnvalue_2)
    (:Is%20Valid
      _)
    (:Is%20Not%20Valid
      (bind _returnvalue_2 (UserInterface|CreateWidget "/Game/BistroBlitz/UI/UI_Fridge.UI_Fridge_C" _returnvalue))))
  (UserInterface|Viewport|AddtoViewport _returnvalue_2 0)
  (Input|SetInputModeUIOnly _returnvalue _returnvalue_2 "DoNotLock" false)
  (Variables|/Script/Engine.PlayerController|SetbShowMouseCursor _returnvalue true))