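; Mop station for Bistro Blitz where players take a mop or put one back.
; Interacting empty-handed spawns a BP_Mop through player controller 0's server call, waits briefly, then assigns the highest-ID mop as the player's holdable.
; Interacting with a held mop sets the holdable to BP_Nothing, while other held items are ignored.
; The prompt offers pickup only to empty hands, otherwise reporting full hands.
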(event Custom|PickUp
  (params (Current%20Player :type BP%20Bistro%20Blitz%20Character%20Object%20Reference) (holding :type Boolean) (holdable :type BP%20Holdable%20Class%20Reference))
  (Variables|Default|SetCurrent%20Player Current%20Player)
  (if holding
    (Utilities|Casting|CastToBP_MopClass holdable)
    (Default|SetHoldableServer (Variables|Default|GetCurrent%20Player) 0 "/Game/BistroBlitz/Blueprints/Holdables/BP_Nothing.BP_Nothing_C" 0 false)
    (else
      (bind _aspc_bistro_blitz (Utilities|Casting|CastToPC_BistroBlitz (Game|GetPlayerController 0)))
      (Default|SpawnActorServer _aspc_bistro_blitz "/Game/BistroBlitz/Blueprints/Holdables/BP_Mop.BP_Mop_C" (Math|Transform|MakeTransform "1000.000000,-50.000000,0.000000"))
      (Utilities|FlowControl|Delay 0.3)
      (Actor|GetAllActorsOfClass "/Game/BistroBlitz/Blueprints/Holdables/BP_Mop.BP_Mop_C")
      (for _array_element 0
        (if (> (Variables|/Game/BistroBlitz/Blueprints/Holdables/BP_Holdable.BP_Holdable_C|GetID _array_element) (Variables|Default|GetHighestID))
          (Variables|Default|SetHighestID (Variables|/Game/BistroBlitz/Blueprints/Holdables/BP_Holdable.BP_Holdable_C|GetID _array_element))))
      (Default|SetHoldableServer (Variables|Default|GetCurrent%20Player) 0 "/Game/BistroBlitz/Blueprints/Holdables/BP_Mop.BP_Mop_C" (Variables|Default|GetHighestID) false))))

(event EventBeginPlay
  (|CallParentFunction) ; This node is disabled and will not be called.\nDrag off pins to build functionality.
)

(event Collision|EventActorBeginOverlap
  (params (OtherActor :type Actor%20Object%20Reference)))

(event EventTick
  (params (DeltaSeconds :type Float%20%28single-precision%29)))

(fn ConstructionScript
  (|CallParentFunction))

(fn Interact
  (params (CurrentHoldable :type BP%20Holdable%20Object%20Reference) (CurrentPlayer :type BP%20Bistro%20Blitz%20Character%20Object%20Reference) (ItemIndex :type Integer) (HoldableType :type BP%20Holdable%20Class%20Reference))
  (|CallParentFunction 0 0 0 0)
  (CallFunction|PickUp CurrentPlayer (Variables|/Game/BistroBlitz/Blueprints/BP_BistroBlitzCharacter.BP_BistroBlitzCharacter_C|GetHolding CurrentPlayer) HoldableType))

(fn GetInteractionInformation
  (params (HeldItem :type BP%20Holdable%20Object%20Reference))
  (bind _isnothing (Default|GetObjectInformation HeldItem))
  (if _isnothing
    (LocalVariables|SetText "Pick up mop")
    (else
      (LocalVariables|SetText "Hands are full")))
  (return (LocalVariables|GetText) true 1.0 false))