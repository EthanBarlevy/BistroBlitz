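; BP_OrderBoard is an interactable Bistro Blitz station where players pin up to eight held orders and take them back oldest first.
; Interact stores order indices in an OrderIDs queue and swaps the player's holdable between BP_Order and BP_Nothing.
; AddOrderServer shows the order's widget in the next slot, and RemoveOrderServer calls RemoveOrderMulti to shift widgets down one.
; GetInteractionInformation builds the prompt from the held item and board occupancy.
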(event Custom|AddOrder%20Server
  (bind _orderids (Variables|Default|GetOrderIDs))
  (bind _returnvalue (Utilities|Array|LastIndex _orderids))
  (bind _holdable_reference (CallFunction|FindHoldable "/Game/BistroBlitz/Blueprints/Holdables/BP_Order.BP_Order_C" (Utilities|Array|Get(acopy) _orderids _returnvalue)))
  (bind _asbp_order (Utilities|Casting|CastToBP_Order _holdable_reference))
  (switch int _returnvalue
    (:0
      (UserInterface|SetWidget (Variables|Default|GetOrder1) (UserInterface|GetWidget (Variables|/Game/BistroBlitz/Blueprints/Holdables/BP_Order.BP_Order_C|GetWidget _asbp_order))))
    (:1
      (UserInterface|SetWidget (Variables|Default|GetOrder2) (UserInterface|GetWidget (Variables|/Game/BistroBlitz/Blueprints/Holdables/BP_Order.BP_Order_C|GetWidget _asbp_order))))
    (:2
      (UserInterface|SetWidget (Variables|Default|GetOrder3) (UserInterface|GetWidget (Variables|/Game/BistroBlitz/Blueprints/Holdables/BP_Order.BP_Order_C|GetWidget _asbp_order))))
    (:3
      (UserInterface|SetWidget (Variables|Default|GetOrder4) (UserInterface|GetWidget (Variables|/Game/BistroBlitz/Blueprints/Holdables/BP_Order.BP_Order_C|GetWidget _asbp_order))))
    (:4
      (UserInterface|SetWidget (Variables|Default|GetOrder5) (UserInterface|GetWidget (Variables|/Game/BistroBlitz/Blueprints/Holdables/BP_Order.BP_Order_C|GetWidget _asbp_order))))
    (:5
      (UserInterface|SetWidget (Variables|Default|GetOrder6) (UserInterface|GetWidget (Variables|/Game/BistroBlitz/Blueprints/Holdables/BP_Order.BP_Order_C|GetWidget _asbp_order))))
    (:6
      (UserInterface|SetWidget (Variables|Default|GetOrder7) (UserInterface|GetWidget (Variables|/Game/BistroBlitz/Blueprints/Holdables/BP_Order.BP_Order_C|GetWidget _asbp_order))))
    (:7
      (UserInterface|SetWidget (Variables|Default|GetOrder8) (UserInterface|GetWidget (Variables|/Game/BistroBlitz/Blueprints/Holdables/BP_Order.BP_Order_C|GetWidget _asbp_order))))))

(event Custom|RemoveOrder%20Server
  (CallFunction|RemoveOrderMulti))

(event Custom|RemoveOrder%20Multi
  (bind _order2 (Variables|Default|GetOrder2))
  (bind _order3 (Variables|Default|GetOrder3))
  (bind _order4 (Variables|Default|GetOrder4))
  (bind _order5 (Variables|Default|GetOrder5))
  (bind _order6 (Variables|Default|GetOrder6))
  (bind _order7 (Variables|Default|GetOrder7))
  (bind _order8 (Variables|Default|GetOrder8))
  (Utilities|FlowControl|Sequence
    (:then_0
      (UserInterface|SetWidget (Variables|Default|GetOrder1) (UserInterface|GetWidget _order2)))
    (:then_1
      (UserInterface|SetWidget _order2 (UserInterface|GetWidget _order3)))
    (:then_2
      (UserInterface|SetWidget _order3 (UserInterface|GetWidget _order4)))
    (:then_3
      (UserInterface|SetWidget _order4 (UserInterface|GetWidget _order5)))
    (:then_4
      (UserInterface|SetWidget _order5 (UserInterface|GetWidget _order6)))
    (:then_5
      (UserInterface|SetWidget _order6 (UserInterface|GetWidget _order7)))
    (:then_6
      (UserInterface|SetWidget _order7 (UserInterface|GetWidget _order8)))
    (:then_7
      (UserInterface|SetWidget _order8 0))))

(event EventBeginPlay
  (|CallParentFunction) ; This node is disabled and will not be called.\nDrag off pins to build functionality.
)

(event Collision|EventActorBeginOverlap
  (params (OtherActor :type Actor%20Object%20Reference)))

(event EventTick
  (params (DeltaSeconds :type Float%20%28single-precision%29))
  (|CallParentFunction DeltaSeconds))

(fn ConstructionScript
  (|CallParentFunction))

(fn Interact
  (params (CurrentHoldable :type BP%20Holdable%20Object%20Reference) (CurrentPlayer :type BP%20Bistro%20Blitz%20Character%20Object%20Reference) (ItemIndex :type Integer) (HoldableType :type BP%20Holdable%20Class%20Reference))
  (bind _orderids (Variables|Default|GetOrderIDs))
  (|CallParentFunction CurrentHoldable CurrentPlayer ItemIndex 0)
  (CallFunction|FindHoldable 0 ItemIndex)
  (LocalVariables|SetNewLocalVar CurrentPlayer)
  (LocalVariables|SetNewLocalVar_0 ItemIndex)
  (if (== HoldableType "/Game/BistroBlitz/Blueprints/Holdables/BP_Order.BP_Order_C")
    (if (< (Utilities|Array|Length (Variables|Default|GetOrderIDs)) 8)
      (Utilities|Array|Add (Variables|Default|GetOrderIDs) (LocalVariables|GetNewLocalVar_0))
      (CallFunction|AddOrderServer)
      (Default|SetHoldableServer (LocalVariables|GetNewLocalVar) 0 "/Game/BistroBlitz/Blueprints/Holdables/BP_Nothing.BP_Nothing_C" 0 true)
      (Variables|/Game/BistroBlitz/Blueprints/BP_BistroBlitzCharacter.BP_BistroBlitzCharacter_C|SetHolding (LocalVariables|GetNewLocalVar) false))
    (elif (== HoldableType "/Game/BistroBlitz/Blueprints/Holdables/BP_Nothing.BP_Nothing_C")
      (if (> (Utilities|Array|Length _orderids) 0)
        (CallFunction|RemoveOrderServer)
        (Default|SetHoldableServer (LocalVariables|GetNewLocalVar) 0 "/Game/BistroBlitz/Blueprints/Holdables/BP_Order.BP_Order_C" (Utilities|Array|Get(acopy) _orderids) false)
        (Utilities|Array|RemoveIndex (Variables|Default|GetOrderIDs))))))

(fn GetInteractionInformation
  (params (HeldItem :type BP%20Holdable%20Object%20Reference))
  (bind _orderids (Variables|Default|GetOrderIDs))
  (bind _returnvalue (Utilities|Array|Length _orderids))
  (bind (_canbecut _hasbeencut _canbecooked _hasbeencooked _isplate _ispan _isnothing _ismop _isorder _hasfood _objectname) (Default|GetObjectInformation HeldItem))
  (if _isorder
    (if (>= _returnvalue 8)
      (LocalVariables|SetText "Order board is full")
      (else
        (LocalVariables|SetText "Place order onto board")))
    (elif _isnothing
      (if (> _returnvalue 0)
        (LocalVariables|SetText "Remove order from board")
        (else
          (LocalVariables|SetText "Order board is empty")))
      (else
        (bind _output_get (LocalVariables|SetText "Can't place "))
        (LocalVariables|SetText (Utilities|String|Append (Utilities|String|Append _output_get (Utilities|String|ToString(Name) _objectname)) " on the order board")))))
  (return (Utilities|Text|ToText(String) (LocalVariables|GetText)) true 1.0 false))