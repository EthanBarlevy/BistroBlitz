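; BP_Fuse is an interactable fuse station in Bistro Blitz that switches power on and off with an animated lever.
; Interacting calls Flip, which plays or reverses a timeline rotating the lever mesh's roll, then toggles PowerState and fires the PowerOn or TurnOff dispatcher.
; The animation direction reads PowerState before it toggles, and the interaction prompt text follows the current state.
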(event Custom|AnimateLever
  (if (Variables|Default|GetPowerState)
    (bind _rotation (Timeline|Timeline PlayFromStart)
      (:Update
        (Transformation|SetRelativeRotation (Variables|Default|GetStaticMesh1) (Math|Rotator|MakeRotator _rotation 0.0 0.0) false false)))
    (else
      (Timeline|Timeline ReverseFromEnd))))

(event EventTick
  (params (DeltaSeconds :type Float%20%28single-precision%29))
  (|CallParentFunction DeltaSeconds))

(fn ConstructionScript
  (|CallParentFunction))

(fn Interact
  (params (CurrentHoldable :type BP%20Holdable%20Object%20Reference) (CurrentPlayer :type BP%20Bistro%20Blitz%20Character%20Object%20Reference) (ItemIndex :type Integer) (HoldableType :type BP%20Holdable%20Class%20Reference))
  (|CallParentFunction CurrentHoldable CurrentPlayer ItemIndex HoldableType)
  (CallFunction|Flip))

(fn ChangeState
  (bind _output_get (Variables|Default|SetPowerState (not (Variables|Default|GetPowerState))))
  (if _output_get
    (Default|CallPoweron)
    (else
      (Default|CallTurnOff))))

(fn Flip
  (CallFunction|AnimateLever)
  (CallFunction|ChangeState))

(fn GetInteractionInformation
  (params (HeldItem :type BP%20Holdable%20Object%20Reference))
  (if (Variables|Default|GetPowerState)
    (LocalVariables|SetText "Turn power off")
    (else
      (LocalVariables|SetText "Turn power on")))
  (return (LocalVariables|GetText) true 1.0 false))