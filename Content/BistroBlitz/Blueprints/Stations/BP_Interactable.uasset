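; BP_Interactable is a base station for Bistro Blitz, with empty interaction functions and default prompt info, apparently meant for child overrides.
; The Interacted event forwards the held item and player to Interact, and FindHoldable looks up a holdable by class and ID.
; A gated Tick sets the owner to the character with PersonalID 1, then closes.
; Overlap-based prompt toggling, interactable assignment and replication ownership are disconnected.
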(event OnComponentBeginOverlap(InteractDistance)
  (params (OverlappedComponent :type Primitive%20Component%20Object%20Reference) (OtherActor :type Actor%20Object%20Reference) (OtherComp :type Primitive%20Component%20Object%20Reference) (OtherBodyIndex :type Integer) (bFromSweep :type Boolean) (SweepResult :type Hit%20Result%20Structure%20%28by%20ref%29))
  ;[0.03646 0.03646 0.03646] Toggle visibility when entering and exiting the area around the station
)

(event OnComponentEndOverlap(InteractDistance)
  (params (OverlappedComponent :type Primitive%20Component%20Object%20Reference) (OtherActor :type Actor%20Object%20Reference) (OtherComp :type Primitive%20Component%20Object%20Reference) (OtherBodyIndex :type Integer))
  ;[0.03646 0.03646 0.03646] Toggle visibility when entering and exiting the area around the station
)

(event Custom|Interacted
  (params (CurrentHoldable :type BP%20Holdable%20Object%20Reference) (CurrentPlayer :type BP%20Bistro%20Blitz%20Character%20Object%20Reference) (ItemIndex :type Integer) (HoldableType :type BP%20Holdable%20Class%20Reference))
  (CallFunction|Interact CurrentHoldable CurrentPlayer ItemIndex HoldableType))

(event Custom|Interact2)

(event EventBeginPlay)

(event EventTick
  (params (DeltaSeconds :type Float%20%28single-precision%29))
  (Utilities|FlowControl|Gate false :!label _label
    (:Exit
      (bind _outactors (Actor|GetAllActorsOfClass "/Game/BistroBlitz/Blueprints/BP_BistroBlitzCharacter.BP_BistroBlitzCharacter_C"))
      (for _array_element _outactors
        (if (== (Variables|/Game/BistroBlitz/Blueprints/BP_BistroBlitzCharacter.BP_BistroBlitzCharacter_C|GetPersonalID _array_element) 1)
          (Actor|SetOwner _array_element)
          (goto _label Close))))))

(fn ConstructionScript)

(fn Interact
  (params (CurrentHoldable :type BP%20Holdable%20Object%20Reference) (CurrentPlayer :type BP%20Bistro%20Blitz%20Character%20Object%20Reference) (ItemIndex :type Integer) (HoldableType :type BP%20Holdable%20Class%20Reference)))

(fn InteractNoRep
  (params (character :type BP%20Bistro%20Blitz%20Character%20Object%20Reference) (holdable :type BP%20Holdable%20Object%20Reference) (ItemIndex :type Integer) (HoldableType :type BP%20Holdable%20Class%20Reference)))

(fn FindHoldable
  (params (Holdable%20Class :type BP%20Holdable%20Class%20Reference) (Index :type Integer))
  (bind _outactors (Actor|GetAllActorsOfClass Holdable%20Class))
  (for _array_element _outactors
    (if (== (Variables|/Game/BistroBlitz/Blueprints/Holdables/BP_Holdable.BP_Holdable_C|GetID _array_element) Index)
      (return _array_element))))

(fn GetInteractionInformation
  (params (HeldItem :type BP%20Holdable%20Object%20Reference))
  (return "" false 0.0 false))