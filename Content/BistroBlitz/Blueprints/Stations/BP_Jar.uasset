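; BP_Jar is a station in BistroBlitz that shows the total money earned when a player looks to interact with it.
; On BeginPlay it finds BP_GameManager and binds to its money-changed event, caching TotalMoneyEarned whenever that fires.
; GetInteractionInformation returns only flavor text: a dollar sign followed by the cached amount rounded to cents, with no radial progress.
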(event Custom|money
  (Variables|Default|SetMoneyEarned (Variables|/Game/BistroBlitz/Blueprints/BP_GameManager.BP_GameManager_C|GetTotalMoneyEarned (stale EventBeginPlay _returnvalue))))

(event EventBeginPlay
  (bind _returnvalue (Actor|GetActorOfClass "/Game/BistroBlitz/Blueprints/BP_GameManager.BP_GameManager_C"))
  (EventDispatchers|BindEventtoMoneyChanged _returnvalue (delegate Custom|money)))

(fn ConstructionScript
  (|CallParentFunction))

(fn GetInteractionInformation
  (params (HeldItem :type BP%20Holdable%20Object%20Reference))
  (return (Utilities|Text|ToText(String) (Utilities|String|Append (Utilities|String|MakeLiteralString "$") (Utilities|String|ToString(Float) (/ (Math|Conversions|ToFloat(Integer) (Math|Float|Round (* (Variables|Default|GetMoneyEarned) 1e+02))) 1e+02)))) false 0.0 true))