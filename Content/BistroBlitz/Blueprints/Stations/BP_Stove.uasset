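; BP_Stove is an interactable kitchen station where players place a pan, cook food in it and take the results.
; Interact handles these hand-offs by held item and stove state, using BP_Nothing for empty.
; Tick advances cooking at the food's own rate until done.
; A server-to-multicast event updates the food mesh, OnRep_Pan sets the pan mesh, and GetInteractionInformation builds the prompt and radial progress.
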(event Custom|AddItem%20Server
  (params (Holdable%20Class :type BP%20Holdable%20Class%20Reference) (Index :type Integer))
  (CallFunction|AddItemMulti Holdable%20Class Index))

(event Custom|AddItem%20Multi
  (params (Holdable%20Class :type BP%20Holdable%20Class%20Reference) (Index :type Integer))
  (bind _holdable_reference (CallFunction|FindHoldable Holdable%20Class Index))
  (Utilities|FlowControl|Delay 0.2)
  (Components|StaticMesh|SetStaticMesh (Variables|Default|Getcooked) (Variables|/Script/Engine.StaticMeshComponent|GetStaticMesh (Variables|/Game/BistroBlitz/Blueprints/Holdables/BP_Holdable.BP_Holdable_C|GetStaticMesh _holdable_reference))))

(event EventBeginPlay
  (|CallParentFunction) ; This node is disabled and will not be called.\nDrag off pins to build functionality.
)

(event Collision|EventActorBeginOverlap
  (params (OtherActor :type Actor%20Object%20Reference))
  (|CallParentFunction OtherActor) ; This node is disabled and will not be called.\nDrag off pins to build functionality.
)

(event EventTick
  (params (DeltaSeconds :type Float%20%28single-precision%29))
  (|CallParentFunction DeltaSeconds)
  (if (and (Variables|Default|GetHasFood) (not (Variables|Default|GetIsDone)))
    (Class|CompoundOperatorsBPLibrary|AddtoDoubleDouble (Variables|Default|GetInteraction%20Total) (* (Variables|Default|GetInteraction%20Amount) DeltaSeconds))
    (bind _output_get (Variables|Default|SetInteraction%20Total (Math|Float|Min(Float) (Variables|Default|GetInteraction%20Total) 1.0)))
    (if (== _output_get 1.0)
      (Variables|Default|SetIsDone true))))

(fn ConstructionScript
  (|CallParentFunction))

(fn Interact
  (params (CurrentHoldable :type BP%20Holdable%20Object%20Reference) (CurrentPlayer :type BP%20Bistro%20Blitz%20Character%20Object%20Reference) (ItemIndex :type Integer) (HoldableType :type BP%20Holdable%20Class%20Reference))
  (LocalVariables|SetNewLocalVar CurrentPlayer)
  (bind _output_get (LocalVariables|SetNewLocalVar_0 ItemIndex))
  (bind _output_get_2 (LocalVariables|SetNewLocalVar_1 HoldableType))
  (bind _holdable_reference (CallFunction|FindHoldable _output_get_2 _output_get))
  (LocalVariables|SetNewLocalVar_2 _holdable_reference)
  (|CallParentFunction 0 0 0 0)
  (if (Variables|Default|GetHasPan)
    (if (Variables|/Game/BistroBlitz/Blueprints/BP_BistroBlitzCharacter.BP_BistroBlitzCharacter_C|GetHolding (LocalVariables|GetNewLocalVar))
      ;[0.03646 0.03646 0.03646] Place a cookable on the pan
      (if (Variables|/Game/BistroBlitz/Blueprints/Holdables/BP_Holdable.BP_Holdable_C|GetCanBeCooked (LocalVariables|GetNewLocalVar_2))
        (Default|SetCookedServer (LocalVariables|GetNewLocalVar_2) true)
        (CallFunction|AddItemServer (LocalVariables|GetNewLocalVar_1) (LocalVariables|GetNewLocalVar_0))
        (Variables|Default|SetFood (LocalVariables|GetNewLocalVar_2))
        (Variables|Default|SetInteraction%20Amount (Variables|/Game/BistroBlitz/Blueprints/Holdables/BP_Holdable.BP_Holdable_C|GetInteractAmount (LocalVariables|GetNewLocalVar_2)))
        (Variables|Default|SetHasFood true)
        (Default|SetHolding (LocalVariables|GetNewLocalVar) 0 "/Game/BistroBlitz/Blueprints/Holdables/BP_Nothing.BP_Nothing_C" 0 false)
        (Audio|PlaySoundatLocation "/Game/BistroBlitz/Audio/sizzle_Cue.sizzle_Cue" (Transformation|GetActorLocation) "0, 0, 0" 1.0 1.0 0.0 0 0 0 0))
      (elif (Variables|Default|GetHasFood)
        ;[0.03646 0.03646 0.03646] Take cooked food
        (if (Variables|Default|GetIsDone)
          (CallFunction|AddItemServer "/Game/BistroBlitz/Blueprints/Holdables/BP_Nothing.BP_Nothing_C")
          (Variables|Default|SetHasFood false)
          (Default|SetHolding (LocalVariables|GetNewLocalVar) 0 (Utilities|GetClass (Variables|Default|GetFood)) (Variables|/Game/BistroBlitz/Blueprints/Holdables/BP_Holdable.BP_Holdable_C|GetID (Variables|Default|GetFood)) false)
          (Variables|Default|SetInteraction%20Total 0.0)
          (Variables|Default|SetIsDone false))
        (else
          ;[0.03646 0.03646 0.03646] Take pan
          (Variables|Default|SetHasPan false)
          (Default|SetHolding (LocalVariables|GetNewLocalVar) 0 "/Game/BistroBlitz/Blueprints/Holdables/BP_Pan.BP_Pan_C" (Variables|/Game/BistroBlitz/Blueprints/Holdables/BP_Holdable.BP_Holdable_C|GetID (Variables|Default|GetPan)) false)
          (bind _returnvalue (Actor|GetActorOfClass "/Game/BistroBlitz/Blueprints/Holdables/BP_Nothing.BP_Nothing_C"))
          (Variables|Default|SetPan _returnvalue))))
    (elif (Variables|/Game/BistroBlitz/Blueprints/BP_BistroBlitzCharacter.BP_BistroBlitzCharacter_C|GetHolding (LocalVariables|GetNewLocalVar))
      ;[0.03646 0.03646 0.03646] Place pan on stove
      (bind _asbp_pan (Utilities|Casting|CastToBP_Pan (LocalVariables|GetNewLocalVar_2)))
      (Variables|Default|SetPan _asbp_pan)
      (Variables|Default|SetHasPan true)
      (Default|SetHolding (LocalVariables|GetNewLocalVar) 0 "/Game/BistroBlitz/Blueprints/Holdables/BP_Nothing.BP_Nothing_C" 0 false))))

(fn OnRepPan
  (Components|StaticMesh|SetStaticMesh (Variables|Default|GetPacedObject) (Variables|/Script/Engine.StaticMeshComponent|GetStaticMesh (Variables|/Game/BistroBlitz/Blueprints/Holdables/BP_Holdable.BP_Holdable_C|GetStaticMesh (Variables|Default|GetPan)))))

(fn GetInteractionInformation
  (params (HeldItem :type BP%20Holdable%20Object%20Reference))
  (bind _isdone (Variables|Default|GetIsDone))
  (bind _food (Variables|Default|GetFood))
  (bind _hasfood (Variables|Default|GetHasFood))
  (bind _name (Variables|/Game/BistroBlitz/Blueprints/Holdables/BP_Holdable.BP_Holdable_C|GetName _food))
  (bind _returnvalue (Utilities|String|ToString(Name) _name))
  (bind (_canbecut _hasbeencut _canbecooked _hasbeencooked _isplate _ispan _isnothing _ismop _isorder _hasfood_2 _objectname) (Default|GetObjectInformation HeldItem))
  (if (Variables|Default|GetHasPan)
    (if _canbecooked
      (if _hasbeencooked
        (LocalVariables|SetText (Utilities|String|Append (Utilities|String|ToString(Name) _objectname) " can't be cooked") :!label _label)
        (else
          (bind _output_get (LocalVariables|SetText "Cook "))
          (LocalVariables|SetText (Utilities|String|Append _output_get (Utilities|String|ToString(Name) _objectname)))))
      (elif _isnothing
        (if _hasfood
          (if _isdone
            (bind _output_get_2 (LocalVariables|SetText "Take "))
            (LocalVariables|SetText (Utilities|String|Append _output_get_2 _returnvalue))
            (else
              (LocalVariables|SetText (Utilities|String|Append _returnvalue " is cooking") :!label _label_2)))
          (else
            (LocalVariables|SetText "Take pan off stove")))
        (elif _hasfood
          (if _isdone
            (LocalVariables|SetText "Hands are full")
            (else
              (goto _label_2)))
          (else
            (goto _label)))))
    (elif _ispan
      (LocalVariables|SetText "Place pan on stove")
      (else
        (LocalVariables|SetText "No pan on stove"))))
  (return (Utilities|Text|ToText(String) (LocalVariables|GetText)) false (Variables|Default|GetInteraction%20Total) false))