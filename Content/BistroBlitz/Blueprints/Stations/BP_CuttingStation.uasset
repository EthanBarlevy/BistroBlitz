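; Cutting station for the Bistro Blitz kitchen, where players place an uncut, cuttable item and chop it through repeated interactions.
; Each chop adds the item's InteractAmount to a progress value that decays per tick; once full, the next empty-handed interaction marks it cut and returns it.
; A BP_Nothing actor represents empty hands, and OnRep_PlacedItem updates the board's mesh.
; GetInteractionInformation supplies prompt text and radial progress.
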(event EventTick
  (params (DeltaSeconds :type Float%20%28single-precision%29))
  (|CallParentFunction DeltaSeconds)
  (if (Variables|Default|GetHasItem)
    (Class|CompoundOperatorsBPLibrary|SubtracttoDoubleDouble (Variables|Default|GetTotalInteractionAmount) 0.005)
    (Variables|Default|SetTotalInteractionAmount (Math|Float|Max(Float) (Variables|Default|GetTotalInteractionAmount) 0.0))))

(fn ConstructionScript
  (|CallParentFunction))

(fn Interact
  (params (CurrentHoldable :type BP%20Holdable%20Object%20Reference) (CurrentPlayer :type BP%20Bistro%20Blitz%20Character%20Object%20Reference) (ItemIndex :type Integer) (HoldableType :type BP%20Holdable%20Class%20Reference))
  (bind _placeditem (Variables|Default|GetPlacedItem))
  (bind _interactincrease (Variables|Default|GetInteractIncrease))
  (LocalVariables|SetHoldable CurrentHoldable)
  (LocalVariables|SetCharacter CurrentPlayer)
  (|CallParentFunction 0 0 0 0)
  (if (Variables|Default|GetHasItem)
    (CallFunction|SetInteractAmount))
  ;[0.03646 0.03646 0.03646] Check if player is holding something
  (bind _returnvalue (Actor|GetActorOfClass "/Game/BistroBlitz/Blueprints/Holdables/BP_Nothing.BP_Nothing_C"))
  (if (!= _returnvalue (LocalVariables|GetHoldable))
    (CallFunction|SetItemonTable (Variables|Default|GetPlacedItem) (LocalVariables|GetCharacter) ItemIndex HoldableType)
    (elif (Variables|Default|GetHasItem)
      (if (Variables|Default|GetisDone)
        (Default|SetCutServer (Variables|Default|GetPlacedItem) true)
        (CallFunction|TakeItemfromTable (LocalVariables|GetCharacter) 0 (Utilities|GetClass _placeditem) (Variables|/Game/BistroBlitz/Blueprints/Holdables/BP_Holdable.BP_Holdable_C|GetID _placeditem))
        (Variables|Default|SetTotalInteractionAmount 0.0)
        (else
          (Class|CompoundOperatorsBPLibrary|AddtoDoubleDouble (Variables|Default|GetTotalInteractionAmount) _interactincrease)
          (if (> _interactincrease 0.0)
            (Audio|PlaySoundatLocation "/Game/BistroBlitz/Audio/cut_Cue.cut_Cue" (Transformation|GetActorLocation) "0, 0, 0" 1.0 1.0 0.0 0 0 0 0)
            (bind _output_get (Variables|Default|SetTotalInteractionAmount (Math|Float|Min(Float) (Variables|Default|GetTotalInteractionAmount) 1.0)))
            (if (== _output_get 1.0)
              (Variables|Default|SetisDone true))))))))

(fn SetInteractAmount
  (Variables|Default|SetInteractIncrease (Variables|/Game/BistroBlitz/Blueprints/Holdables/BP_Holdable.BP_Holdable_C|GetInteractAmount (Variables|Default|GetPlacedItem))))

(fn SetItemonTable
  (params (holdable :type BP%20Holdable%20Object%20Reference) (player :type BP%20Bistro%20Blitz%20Character%20Object%20Reference) (ItemIndex :type Integer) (HoldableType :type BP%20Holdable%20Class%20Reference))
  (bind _holdable_reference (CallFunction|FindHoldable HoldableType ItemIndex))
  (LocalVariables|SetNewLocalVar _holdable_reference)
  (if (and (not (Variables|/Game/BistroBlitz/Blueprints/Holdables/BP_Holdable.BP_Holdable_C|GetCut _holdable_reference)) (Variables|/Game/BistroBlitz/Blueprints/Holdables/BP_Holdable.BP_Holdable_C|GetCanBeCut _holdable_reference))
    (Variables|Default|SetPlacedItem (LocalVariables|GetNewLocalVar))
    (Default|SetHoldableServer player 0 "/Game/BistroBlitz/Blueprints/Holdables/BP_Nothing.BP_Nothing_C" 0 false)
    (Variables|Default|SetHasItem true)))

(fn TakeItemfromTable
  (params (character :type BP%20Bistro%20Blitz%20Character%20Object%20Reference) (holdable :type BP%20Holdable%20Object%20Reference) (HoldableClass :type BP%20Holdable%20Class%20Reference) (Index :type Integer))
  (Default|SetHoldableServer character 0 HoldableClass Index false)
  (bind _returnvalue (Actor|GetActorOfClass "/Game/BistroBlitz/Blueprints/Holdables/BP_Nothing.BP_Nothing_C"))
  (Variables|Default|SetPlacedItem _returnvalue)
  (Variables|Default|SetHasItem false)
  (Variables|Default|SetisDone false))

(fn OnRepPlacedItem
  (Components|StaticMesh|SetStaticMesh (Variables|Default|GetPlaced%20Object) (Variables|/Script/Engine.StaticMeshComponent|GetStaticMesh (Variables|/Game/BistroBlitz/Blueprints/Holdables/BP_Holdable.BP_Holdable_C|GetStaticMesh (Variables|Default|GetPlacedItem)))))

(fn InteractNoRep
  (params (character :type BP%20Bistro%20Blitz%20Character%20Object%20Reference) (holdable :type BP%20Holdable%20Object%20Reference) (ItemIndex :type Integer) (HoldableType :type BP%20Holdable%20Class%20Reference))
  (|CallParentFunction character holdable 0 0))

(fn GetInteractionInformation
  (params (HeldItem :type BP%20Holdable%20Object%20Reference))
  (bind (_canbecut _hasbeencut _canbecooked _hasbeencooked _isplate _ispan _isnothing _ismop _isorder _hasfood _objectname) (Default|GetObjectInformation HeldItem))
  (if (Variables|Default|GetHasItem)
    (bind _output_get (LocalVariables|SetText "Cut "))
    (LocalVariables|SetText (Utilities|String|Append _output_get (Utilities|String|ToString(Name) (Variables|/Game/BistroBlitz/Blueprints/Holdables/BP_Holdable.BP_Holdable_C|GetName (Variables|Default|GetPlacedItem)))))
    (elif _canbecut
      (if _hasbeencut
        (bind _output_get_2 (LocalVariables|SetText "Can't cut " :!label _label))
        (LocalVariables|SetText (Utilities|String|Append _output_get_2 (Utilities|String|ToString(Name) _objectname)))
        (else
          (bind _output_get_3 (LocalVariables|SetText "Place "))
          (LocalVariables|SetText (Utilities|String|Append (Utilities|String|Append _output_get_3 (Utilities|String|ToString(Name) _objectname)) " on cutting board"))))
      (elif _isnothing
        (LocalVariables|SetText "Nothing to cut")
        (else
          (goto _label)))))
  (return (Utilities|Text|ToText(String) (LocalVariables|GetText)) false (Variables|Default|GetTotalInteractionAmount) false))