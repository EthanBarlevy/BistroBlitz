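; BP_Sink is a kitchen station that hands a new plate to an empty-handed player, with no limit on supply.
; Interact forwards to an event that spawns BP_Plate at a fixed location through player controller 0's server spawn call.
; After a short delay it finds the highest plate ID and sets that plate as the player's holdable via a server call.
; GetInteractionInformation supplies the grab or hands-full prompt.
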(event Custom|Interac
  (params (CurrentHoldable :type BP%20Holdable%20Object%20Reference) (CurrentPlayer :type BP%20Bistro%20Blitz%20Character%20Object%20Reference))
  ;[0.03646 0.03646 0.03646] Currently just spawns a plate. I will need to change this to only give out so many clean plates if I add plate washing later
  (if (not (Variables|/Game/BistroBlitz/Blueprints/BP_BistroBlitzCharacter.BP_BistroBlitzCharacter_C|GetHolding CurrentPlayer))
    (bind _aspc_bistro_blitz (Utilities|Casting|CastToPC_BistroBlitz (Game|GetPlayerController 0)))
    (Default|SpawnActorServer _aspc_bistro_blitz "/Game/BistroBlitz/Blueprints/Holdables/BP_Plate.BP_Plate_C" (Math|Transform|MakeTransform "1000.000000,-50.000000,0.000000"))
    (Utilities|FlowControl|Delay 0.3)
    (bind _outactors (Actor|GetAllActorsOfClass "/Game/BistroBlitz/Blueprints/Holdables/BP_Plate.BP_Plate_C"))
    (for _array_element _outactors
      (if (> (Variables|/Game/BistroBlitz/Blueprints/Holdables/BP_Holdable.BP_Holdable_C|GetID _array_element) (Variables|Default|GetHighestID))
        (Variables|Default|SetHighestID (Variables|/Game/BistroBlitz/Blueprints/Holdables/BP_Holdable.BP_Holdable_C|GetID _array_element))))
    (Default|SetHoldableServer CurrentPlayer 0 "/Game/BistroBlitz/Blueprints/Holdables/BP_Plate.BP_Plate_C" (Variables|Default|GetHighestID) false)))

(event EventBeginPlay
  (|CallParentFunction) ; This node is disabled and will not be called.\nDrag off pins to build functionality.
)

(event Collision|EventActorBeginOverlap
  (params (OtherActor :type Actor%20Object%20Reference))
  (|CallParentFunction OtherActor) ; This node is disabled and will not be called.\nDrag off pins to build functionality.
)

(event EventTick
  (params (DeltaSeconds :type Float%20%28single-precision%29))
  (|CallParentFunction DeltaSeconds) ; This node is disabled and will not be called.\nDrag off pins to build functionality.
)

(fn ConstructionScript
  (|CallParentFunction))

(fn Interact
  (params (CurrentHoldable :type BP%20Holdable%20Object%20Reference) (CurrentPlayer :type BP%20Bistro%20Blitz%20Character%20Object%20Reference) (ItemIndex :type Integer) (HoldableType :type BP%20Holdable%20Class%20Reference))
  (|CallParentFunction 0 0 0 0)
  (CallFunction|Interac CurrentHoldable CurrentPlayer))

(fn GetInteractionInformation
  (params (HeldItem :type BP%20Holdable%20Object%20Reference))
  (bind _isnothing (Default|GetObjectInformation HeldItem))
  (if _isnothing
    (LocalVariables|SetText "Grab plate from sink")
    (else
      (LocalVariables|SetText "Hands are full")))
  (return (LocalVariables|GetText) true 1.0 false))