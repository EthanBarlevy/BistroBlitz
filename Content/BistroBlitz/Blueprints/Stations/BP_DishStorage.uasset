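; BP_DishStorage is an interactable counter station in Bistro Blitz that holds up to three plates with food for players to take.
; Interact stores a held plate's index in Dishes or hands back the oldest, relaying changes through server-to-multicast events that update three mesh slots.
; Removal takes the first array entry but blanks the last occupied slot's mesh, without shifting the others.
; GetInteractionInformation supplies context-sensitive prompt text.
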(event OnComponentBeginOverlap(InteractDistance)
  (params (OverlappedComponent :type Primitive%20Component%20Object%20Reference) (OtherActor :type Actor%20Object%20Reference) (OtherComp :type Primitive%20Component%20Object%20Reference) (OtherBodyIndex :type Integer) (bFromSweep :type Boolean) (SweepResult :type Hit%20Result%20Structure%20%28by%20ref%29))
  (Utilities|Casting|CastToBP_BistroBlitzCharacter OtherActor)
  (Rendering|ToggleVisibility (Variables|Default|GetInteractPrompt1) false))

(event OnComponentEndOverlap(InteractDistance)
  (params (OverlappedComponent :type Primitive%20Component%20Object%20Reference) (OtherActor :type Actor%20Object%20Reference) (OtherComp :type Primitive%20Component%20Object%20Reference) (OtherBodyIndex :type Integer))
  (Utilities|Casting|CastToBP_BistroBlitzCharacter OtherActor)
  (Rendering|ToggleVisibility (Variables|Default|GetInteractPrompt1) false))

(event Custom|AddItem%20Server
  (params (Holdable%20Class :type BP%20Holdable%20Class%20Reference) (Index :type Integer))
  (CallFunction|AddItemMulti Holdable%20Class Index))

(event Custom|AddItem%20Multi
  (params (Holdable%20Class :type BP%20Holdable%20Class%20Reference) (Index :type Integer))
  (bind _returnvalue (Utilities|Array|Add (Variables|Default|GetDishes) Index))
  (bind _holdable_reference (CallFunction|FindHoldable Holdable%20Class Index))
  (switch int _returnvalue
    (:0
      (Components|StaticMesh|SetStaticMesh (Variables|Default|GetDish1) (Variables|/Script/Engine.StaticMeshComponent|GetStaticMesh (Variables|/Game/BistroBlitz/Blueprints/Holdables/BP_Holdable.BP_Holdable_C|GetStaticMesh _holdable_reference))))
    (:1
      (Components|StaticMesh|SetStaticMesh (Variables|Default|GetDish2) (Variables|/Script/Engine.StaticMeshComponent|GetStaticMesh (Variables|/Game/BistroBlitz/Blueprints/Holdables/BP_Holdable.BP_Holdable_C|GetStaticMesh _holdable_reference))))
    (:2
      (Components|StaticMesh|SetStaticMesh (Variables|Default|GetDish3) (Variables|/Script/Engine.StaticMeshComponent|GetStaticMesh (Variables|/Game/BistroBlitz/Blueprints/Holdables/BP_Holdable.BP_Holdable_C|GetStaticMesh _holdable_reference))))))

(event Custom|RemoveItem%20Server
  (params (Holdable%20Class :type BP%20Holdable%20Class%20Reference) (Index :type Integer))
  (CallFunction|RemoveItemMulti Holdable%20Class Index))

(event Custom|RemoveItem%20Multi
  (params (Holdable%20Class :type BP%20Holdable%20Class%20Reference) (Index :type Integer))
  (bind _holdable_reference (CallFunction|FindHoldable Holdable%20Class Index))
  (switch int (Utilities|Array|Length (Variables|Default|GetDishes))
    (:1
      (Components|StaticMesh|SetStaticMesh (Variables|Default|GetDish1) (Variables|/Script/Engine.StaticMeshComponent|GetStaticMesh (Variables|/Game/BistroBlitz/Blueprints/Holdables/BP_Holdable.BP_Holdable_C|GetStaticMesh _holdable_reference))))
    (:2
      (Components|StaticMesh|SetStaticMesh (Variables|Default|GetDish2) (Variables|/Script/Engine.StaticMeshComponent|GetStaticMesh (Variables|/Game/BistroBlitz/Blueprints/Holdables/BP_Holdable.BP_Holdable_C|GetStaticMesh _holdable_reference))))
    (:3
      (Components|StaticMesh|SetStaticMesh (Variables|Default|GetDish3) (Variables|/Script/Engine.StaticMeshComponent|GetStaticMesh (Variables|/Game/BistroBlitz/Blueprints/Holdables/BP_Holdable.BP_Holdable_C|GetStaticMesh _holdable_reference)))))
  (Utilities|Array|RemoveIndex (Variables|Default|GetDishes)))

(event EventBeginPlay
  (|CallParentFunction))

(fn ConstructionScript
  (|CallParentFunction))

(fn Interact
  (params (CurrentHoldable :type BP%20Holdable%20Object%20Reference) (CurrentPlayer :type BP%20Bistro%20Blitz%20Character%20Object%20Reference) (ItemIndex :type Integer) (HoldableType :type BP%20Holdable%20Class%20Reference))
  (bind _dishes (Variables|Default|GetDishes))
  (LocalVariables|SetNewLocalVar CurrentPlayer)
  (bind _output_get (LocalVariables|SetNewLocalVar_0 ItemIndex))
  (bind _output_get_2 (LocalVariables|SetNewLocalVar_1 HoldableType))
  (bind _holdable_reference (CallFunction|FindHoldable _output_get_2 _output_get))
  (LocalVariables|SetNewLocalVar_2 _holdable_reference)
  (|CallParentFunction 0 0 0 0)
  (if (Variables|/Game/BistroBlitz/Blueprints/BP_BistroBlitzCharacter.BP_BistroBlitzCharacter_C|GetHolding (LocalVariables|GetNewLocalVar))
    (bind _asbp_plate (Utilities|Casting|CastToBP_Plate (LocalVariables|GetNewLocalVar_2)))
    (if (Variables|/Game/BistroBlitz/Blueprints/Holdables/BP_Plate.BP_Plate_C|GetHasFood _asbp_plate)
      (if (< (Utilities|Array|Length (Variables|Default|GetDishes)) 3)
        (CallFunction|AddItemServer "/Game/BistroBlitz/Blueprints/Holdables/BP_Plate.BP_Plate_C" (LocalVariables|GetNewLocalVar_0))
        (Default|SetHolding (LocalVariables|GetNewLocalVar) 0 "/Game/BistroBlitz/Blueprints/Holdables/BP_Nothing.BP_Nothing_C" 0 false)))
    (elif (> (Utilities|Array|Length _dishes) 0)
      (Default|SetHolding (LocalVariables|GetNewLocalVar) 0 "/Game/BistroBlitz/Blueprints/Holdables/BP_Plate.BP_Plate_C" (Utilities|Array|Get(acopy) _dishes) false)
      (CallFunction|RemoveItemServer "/Game/BistroBlitz/Blueprints/Holdables/BP_Nothing.BP_Nothing_C"))))

(fn GetInteractionInformation
  (params (HeldItem :type BP%20Holdable%20Object%20Reference))
  (bind (_canbecut _hasbeencut _canbecooked _hasbeencooked _isplate _ispan _isnothing _ismop _isorder _hasfood _objectname) (Default|GetObjectInformation HeldItem))
  (if _isplate
    (if _hasfood
      (if (>= (Utilities|Array|Length (Variables|Default|GetDishes)) 3)
        (LocalVariables|SetText "Counter is full")
        (else
          (LocalVariables|SetText "Place dish on counter")))
      (else
        (LocalVariables|SetText "Plate must have food")))
    (elif _isnothing
      (if (>= (Utilities|Array|Length (Variables|Default|GetDishes)) 1)
        (LocalVariables|SetText "Take dish from counter")
        (else
          (LocalVariables|SetText "No dishes to take")))
      (else
        (bind _output_get (LocalVariables|SetText "Can't place "))
        (LocalVariables|SetText (Utilities|String|Append (Utilities|String|Append _output_get (Utilities|String|ToString(Name) _objectname)) " on counter")))))
  (return (Utilities|Text|ToText(String) (LocalVariables|GetText)) true 1.0 false))