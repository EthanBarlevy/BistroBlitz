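; Trash can station in Bistro Blitz where players discard the item they are holding.
; Interacting calls the player's SetHoldableServer to replace the held item with BP_Nothing, and the interaction text names that item or says there is nothing to throw away.
; A gated Tick searches for the character with PersonalID 1, makes it the owner, then closes the gate.
; BeginPlay hides the mesh when the Visible flag is off.
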(event EventBeginPlay
  (|CallParentFunction)
  (if (not (Variables|Default|Getvisible))
    (Rendering|SetVisibility (Variables|Default|GetStaticMesh) false false)))

(event EventTick
  (params (DeltaSeconds :type Float%20%28single-precision%29))
  (|CallParentFunction DeltaSeconds)
  (Utilities|FlowControl|Gate false :!label _label
    (:Exit
      (bind _outactors (Actor|GetAllActorsOfClass "/Game/BistroBlitz/Blueprints/BP_BistroBlitzCharacter.BP_BistroBlitzCharacter_C"))
      (for _array_element _outactors
        (if (== (Variables|/Game/BistroBlitz/Blueprints/BP_BistroBlitzCharacter.BP_BistroBlitzCharacter_C|GetPersonalID _array_element) 1)
          (Actor|SetOwner _array_element)
          (goto _label Close))))))

(fn ConstructionScript
  (|CallParentFunction))

(fn Interact
  (params (CurrentHoldable :type BP%20Holdable%20Object%20Reference) (CurrentPlayer :type BP%20Bistro%20Blitz%20Character%20Object%20Reference) (ItemIndex :type Integer) (HoldableType :type BP%20Holdable%20Class%20Reference))
  (|CallParentFunction 0 0 0 0)
  (Default|SetHoldableServer CurrentPlayer 0 "/Game/BistroBlitz/Blueprints/Holdables/BP_Nothing.BP_Nothing_C" 0 true))

(fn GetInteractionInformation
  (params (HeldItem :type BP%20Holdable%20Object%20Reference))
  (bind (_canbecut _hasbeencut _canbecooked _hasbeencooked _isplate _ispan _isnothing _ismop _isorder _hasfood _objectname) (Default|GetObjectInformation HeldItem))
  (if _isnothing
    (LocalVariables|SetText "Nothing to throw away")
    (else
      (bind _output_get (LocalVariables|SetText "Throw away "))
      (LocalVariables|SetText (Utilities|String|Append _output_get (Utilities|String|ToString(Name) _objectname)))))
  (return (Utilities|Text|ToText(String) (LocalVariables|GetText)) true 1.0 false))