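; Interactable mess puddle station in Bistro Blitz that a player cleans up with a mop.
; Interact stores the player and held-item details, runs the parent interaction, then destroys the actor if the held class is BP_Mop.
; The interaction prompt checks the held item's IsMop flag to show either a clean-up or a grab-a-mop message, flagged as a single interaction.
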(event EventTick
  (params (DeltaSeconds :type Float%20%28single-precision%29))
  (|CallParentFunction DeltaSeconds))

(fn ConstructionScript
  (|CallParentFunction))

(fn Interact
  (params (CurrentHoldable :type BP%20Holdable%20Object%20Reference) (CurrentPlayer :type BP%20Bistro%20Blitz%20Character%20Object%20Reference) (ItemIndex :type Integer) (HoldableType :type BP%20Holdable%20Class%20Reference))
  (LocalVariables|Setplayer CurrentPlayer)
  (LocalVariables|Setholding%20index ItemIndex)
  (LocalVariables|Setholding%20class HoldableType)
  (|CallParentFunction 0 CurrentPlayer ItemIndex HoldableType)
  (if (== (LocalVariables|Getholding%20class) "/Game/BistroBlitz/Blueprints/Holdables/BP_Mop.BP_Mop_C")
    (Actor|DestroyActor)))

(fn GetInteractionInformation
  (params (HeldItem :type BP%20Holdable%20Object%20Reference))
  (bind _ismop (Default|GetObjectInformation HeldItem))
  (if _ismop
    (LocalVariables|SetText "Clean up puddle")
    (else
      (LocalVariables|SetText "Grab mop to clean")))
  (return (LocalVariables|GetText) true 1.0 false))