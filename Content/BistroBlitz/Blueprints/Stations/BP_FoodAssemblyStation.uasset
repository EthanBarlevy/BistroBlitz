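; Kitchen station in Bistro Blitz where players place an empty plate, add held items to it, and pick up the dish.
; Interact branches on HasPlate, while RefPlate's OnRep shows the plate mesh and sets that flag.
; AddItemsMulti stacks spawned mesh components by item height, setting each mesh after a short delay.
; RemoveItemsMulti clears the stack on pickup and turns a filled plate into a cloche-covered dish marked as having food.
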(event Custom|AddItems%20Multi
  (bind _holdable_reference (CallFunction|FindHoldable "/Game/BistroBlitz/Blueprints/Holdables/BP_Plate.BP_Plate_C" (Variables|Default|GetPlateIndex)))
  (bind _asbp_plate (Utilities|Casting|CastToBP_Plate _holdable_reference))
  (bind _returnvalue (AddComponent|AddStaticMeshComponent false (Variables|Default|GetLastTransform)))
  (Utilities|Array|Add (Variables|Default|GetMeshes) _returnvalue)
  (Utilities|FlowControl|Delay 0.3)
  (Components|StaticMesh|SetStaticMesh _returnvalue (Variables|/Script/Engine.StaticMeshComponent|GetStaticMesh (Variables|/Game/BistroBlitz/Blueprints/Holdables/BP_Holdable.BP_Holdable_C|GetStaticMesh (Utilities|Array|Get(acopy) (Variables|/Game/BistroBlitz/Blueprints/Holdables/BP_Plate.BP_Plate_C|GetHoldables _asbp_plate) (Utilities|Array|LastIndex (Variables|/Game/BistroBlitz/Blueprints/Holdables/BP_Plate.BP_Plate_C|GetHoldables _asbp_plate))))))
  (Variables|Default|SetLastTransform (Math|Transform|MakeTransform (+ (.location (Variables|Default|GetLastTransform)) (Variables|/Game/BistroBlitz/Blueprints/Holdables/BP_Holdable.BP_Holdable_C|GetHeight (Utilities|Array|Get(acopy) (Variables|/Game/BistroBlitz/Blueprints/Holdables/BP_Plate.BP_Plate_C|GetHoldables _asbp_plate) (Utilities|Array|LastIndex (Variables|/Game/BistroBlitz/Blueprints/Holdables/BP_Plate.BP_Plate_C|GetHoldables _asbp_plate))))) (.rotation (Variables|Default|GetLastTransform)) (.scale (Variables|Default|GetLastTransform)))))

(event Custom|RemoveItems%20Multi
  (bind _meshes (Variables|Default|GetMeshes))
  (for _array_element _meshes
    (Components|DestroyComponent _array_element))
  (Utilities|Array|Clear _meshes)
  (Variables|Default|SetLastTransform (Math|Transform|MakeTransform "0.000000,0.000000,101.000000" "0, 0, 0" "0.350000,0.350000,0.350000"))
  (bind _holdable_reference (CallFunction|FindHoldable "/Game/BistroBlitz/Blueprints/Holdables/BP_Plate.BP_Plate_C" (Variables|Default|GetPlateIndex)))
  (bind _asbp_plate (Utilities|Casting|CastToBP_Plate _holdable_reference))
  (if (> (Utilities|Array|Length (Variables|/Game/BistroBlitz/Blueprints/Holdables/BP_Plate.BP_Plate_C|GetHoldables _asbp_plate)) 0)
    (Components|StaticMesh|SetStaticMesh (Variables|/Game/BistroBlitz/Blueprints/Holdables/BP_Holdable.BP_Holdable_C|GetStaticMesh _asbp_plate) "/Game/BistroBlitz/Models/Cloche2.Cloche2")
    (Variables|/Game/BistroBlitz/Blueprints/Holdables/BP_Plate.BP_Plate_C|SetHasFood _asbp_plate true))
  (Components|StaticMesh|SetStaticMesh (Variables|Default|GetPlacedObject) 0))

(event EventBeginPlay
  (|CallParentFunction) ; This node is disabled and will not be called.\nDrag off pins to build functionality.
)

(event Collision|EventActorBeginOverlap
  (params (OtherActor :type Actor%20Object%20Reference))
  (|CallParentFunction OtherActor) ; This node is disabled and will not be called.\nDrag off pins to build functionality.
)

(event EventTick
  (params (DeltaSeconds :type Float%20%28single-precision%29))
  (|CallParentFunction DeltaSeconds) ; This node is disabled and will not be called.\nDrag off pins to build functionality.
)

(fn ConstructionScript
  (|CallParentFunction))

(fn Interact
  (params (CurrentHoldable :type BP%20Holdable%20Object%20Reference) (CurrentPlayer :type BP%20Bistro%20Blitz%20Character%20Object%20Reference) (ItemIndex :type Integer) (HoldableType :type BP%20Holdable%20Class%20Reference))
  (LocalVariables|SetNewLocalVar CurrentPlayer)
  (LocalVariables|SetNewLocalVar_0 ItemIndex)
  (|CallParentFunction 0 0 0 0)
  (if (Variables|Default|GetHasPlate)
    ;[0.03646 0.03646 0.03646] Add Item to plate
    (if (!= HoldableType "/Game/BistroBlitz/Blueprints/Holdables/BP_Nothing.BP_Nothing_C")
      (bind _holdable_reference (CallFunction|FindHoldable HoldableType (LocalVariables|GetNewLocalVar_0)))
      (bind _output_get (LocalVariables|SetNewLocalVar_1 _holdable_reference))
      (Default|AddItem (Variables|Default|GetRef_Plate) _output_get)
      (CallFunction|AddItemsMulti)
      (Default|SetHolding (LocalVariables|GetNewLocalVar) 0 "/Game/BistroBlitz/Blueprints/Holdables/BP_Nothing.BP_Nothing_C" 0 false)
      (else
        ;[0.03646 0.03646 0.03646] Pick up plate
        (CallFunction|RemoveItemsMulti)
        (Default|SetHolding (LocalVariables|GetNewLocalVar) 0 "/Game/BistroBlitz/Blueprints/Holdables/BP_Plate.BP_Plate_C" (Variables|Default|GetPlateIndex) false)
        (Variables|Default|SetHasPlate false)))
    (else
      ;[0.03646 0.03646 0.03646] Place plate on station
      (if (Variables|/Game/BistroBlitz/Blueprints/BP_BistroBlitzCharacter.BP_BistroBlitzCharacter_C|GetHolding (LocalVariables|GetNewLocalVar))
        (if (== HoldableType "/Game/BistroBlitz/Blueprints/Holdables/BP_Plate.BP_Plate_C")
          (bind _holdable_reference_2 (CallFunction|FindHoldable "/Game/BistroBlitz/Blueprints/Holdables/BP_Plate.BP_Plate_C" (LocalVariables|GetNewLocalVar_0)))
          (LocalVariables|SetNewLocalVar_1 _holdable_reference_2)
          (Variables|Default|SetPlateIndex (LocalVariables|GetNewLocalVar_0))
          (bind _asbp_plate (Utilities|Casting|CastToBP_Plate (LocalVariables|GetNewLocalVar_1)))
          (if (not (> (Utilities|Array|Length (Variables|/Game/BistroBlitz/Blueprints/Holdables/BP_Plate.BP_Plate_C|GetHoldables _asbp_plate)) 0))
            (Variables|Default|SetRef_Plate _asbp_plate)
            (Default|SetHolding (LocalVariables|GetNewLocalVar) 0 "/Game/BistroBlitz/Blueprints/Holdables/BP_Nothing.BP_Nothing_C" 0 false)))))))

(fn OnRepRefPlate
  (Components|StaticMesh|SetStaticMesh (Variables|Default|GetPlacedObject) (Variables|/Script/Engine.StaticMeshComponent|GetStaticMesh (Variables|/Game/BistroBlitz/Blueprints/Holdables/BP_Holdable.BP_Holdable_C|GetStaticMesh (Variables|Default|GetRef_Plate))))
  (Variables|Default|SetHasPlate true))

(fn GetInteractionInformation
  (params (HeldItem :type BP%20Holdable%20Object%20Reference))
  (bind (_canbecut _hasbeencut _canbecooked _hasbeencooked _isplate _ispan _isnothing _ismop _isorder _hasfood _objectname) (Default|GetObjectInformation HeldItem))
  (if (Variables|Default|GetHasPlate)
    (if _isnothing
      (if (> (Utilities|Array|Length (Variables|Default|GetMeshes)) 0)
        (LocalVariables|SetText "Pick up dish")
        (else
          (LocalVariables|SetText "Pick up plate")))
      (else
        (bind _output_get (LocalVariables|SetText "Add "))
        (LocalVariables|SetText (Utilities|String|Append (Utilities|String|Append _output_get (Utilities|String|ToString(Name) _objectname)) " to dish"))))
    (elif _isplate
      (if _hasfood
        (LocalVariables|SetText "Plate must be empty")
        (else
          (LocalVariables|SetText "Place plate")))
      (else
        (LocalVariables|SetText "No plate on the counter"))))
  (return (Utilities|Text|ToText(String) (LocalVariables|GetText)) true 1.0 false))