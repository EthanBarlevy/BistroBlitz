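; Bistro Blitz table station where players seat a customer, take their order and serve a plated dish.
; Overlap seats the matching customer via AI blackboard keys; Interact either spawns a random BP_Order for the player or places the plate.
; Server/Multi event pairs rebuild the dish as stacked static meshes on the table.
; JudgeDish scores ingredient order with partial credit, prices the order, updates game score and customer happiness, then clears the table.
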(event OnComponentBeginOverlap(InteractDistance)
  (params (OverlappedComponent :type Primitive%20Component%20Object%20Reference) (OtherActor :type Actor%20Object%20Reference) (OtherComp :type Primitive%20Component%20Object%20Reference) (OtherBodyIndex :type Integer) (bFromSweep :type Boolean) (SweepResult :type Hit%20Result%20Structure%20%28by%20ref%29))
  (bind _outactors (Actor|GetAllActorsOfClass "/Game/BistroBlitz/Blueprints/AI/BP_BistroBlitzCustomer.BP_BistroBlitzCustomer_C"))
  (for _array_element _outactors
    (if (== (Variables|/Game/BistroBlitz/Blueprints/AI/BP_BistroBlitzCustomer.BP_BistroBlitzCustomer_C|GetID _array_element) (Variables|Default|GetCustomerID))
      (Variables|Default|SetCustomer _array_element)))
  (bind _asbp_bistro_blitz_customer (Utilities|Casting|CastToBP_BistroBlitzCustomer OtherActor))
  (if (== _asbp_bistro_blitz_customer (Variables|Default|GetCustomer)) ; This seems unneeded but whatever\nprobably an artifact of multiplayer
    (bind _asbp_bbc_aicontroller (Utilities|Casting|CastToBP_BBC_AIController (AI|GetAIController _asbp_bistro_blitz_customer)))
    (AI|Components|Blackboard|SetValueasBool (Variables|/Script/AIModule.AIController|GetBlackboard _asbp_bbc_aicontroller) (Utilities|Name|MakeLiteralName "HasBeenSeated") true)
    (Class|BlackboardComponent|SetValueasInt (Variables|/Script/AIModule.AIController|GetBlackboard _asbp_bbc_aicontroller) (Utilities|Name|MakeLiteralName "TableNumber") (Variables|Default|GetTableNumber))
    (Default|SitServer (Variables|Default|GetCustomer))
    (Variables|Default|SetCustomerID -1)
    (Variables|Default|SetHasCustomer true)
    (else
      (Development|PrintString "no customer??"))))

(event Custom|hold
  (params (Index :type Integer) (Target :type BP%20Bistro%20Blitz%20Character%20Object%20Reference))
  (Default|SetHolding Target 0 "/Game/BistroBlitz/Blueprints/Holdables/BP_Order.BP_Order_C" Index false))

(event Custom|RemoveCloche%20Server
  (params (Holdable%20Class :type BP%20Holdable%20Class%20Reference) (Index :type Integer))
  (CallFunction|RemoveClocheMulti Holdable%20Class Index))

(event Custom|RemoveCloche%20Multi
  (params (Holdable%20Class :type BP%20Holdable%20Class%20Reference) (Index :type Integer))
  (bind _holdable_reference (CallFunction|FindHoldable Holdable%20Class Index))
  (Components|StaticMesh|SetStaticMesh (Variables|/Game/BistroBlitz/Blueprints/Holdables/BP_Holdable.BP_Holdable_C|GetStaticMesh _holdable_reference) "/Game/BistroBlitz/Models/plate-big.plate-big")
  (Components|StaticMesh|SetStaticMesh (Variables|Default|GetPlate) (Variables|/Script/Engine.StaticMeshComponent|GetStaticMesh (Variables|/Game/BistroBlitz/Blueprints/Holdables/BP_Holdable.BP_Holdable_C|GetStaticMesh _holdable_reference))))

(event Custom|CreateMeshes%20Server
  (params (Holdable%20Class :type Array%20of%20BP%20Holdable%20Class%20References) (Index :type Array%20of%20Integers))
  (CallFunction|CreateMeshesMulti Holdable%20Class Index))

(event Custom|CreateMeshes%20Multi
  (params (Holdable%20Class :type Array%20of%20BP%20Holdable%20Class%20References) (Index :type Array%20of%20Integers))
  (for (_array_element _array_index) Holdable%20Class
    (bind _holdable_reference (CallFunction|FindHoldable _array_element (Utilities|Array|Get(acopy) Index _array_index)))
    (bind _returnvalue (AddComponent|AddStaticMeshComponent false (Variables|Default|GetLastTransform)))
    (Collision|SetCollisionEnabled _returnvalue "NoCollision")
    (Utilities|Array|Add (Variables|Default|GetMeshes) _returnvalue)
    (Components|StaticMesh|SetStaticMesh _returnvalue (Variables|/Script/Engine.StaticMeshComponent|GetStaticMesh (Variables|/Game/BistroBlitz/Blueprints/Holdables/BP_Holdable.BP_Holdable_C|GetStaticMesh _holdable_reference)))
    (Variables|Default|SetLastTransform (Math|Transform|MakeTransform (+ (Variables|/Game/BistroBlitz/Blueprints/Holdables/BP_Holdable.BP_Holdable_C|GetHeight _holdable_reference) (.location (Variables|Default|GetLastTransform))) (.rotation (Variables|Default|GetLastTransform)) (.scale (Variables|Default|GetLastTransform))))))

(event Custom|RemoveMeshes%20Server)

(event Custom|RemoveMeshes%20Multi)

(event Custom|JudgeDishServer
  (CallFunction|JudgeDish))

(event Custom|remove%20dish%20multi
  (CallFunction|RemoveDish))

(event Custom|do%20order
  (params (Character :type BP%20Bistro%20Blitz%20Character%20Object%20Reference))
  (Utilities|FlowControl|Delay 0.2)
  (bind _outactors (Actor|GetAllActorsOfClass "/Game/BistroBlitz/Blueprints/Holdables/BP_Order.BP_Order_C"))
  (for _array_element _outactors
    (if (> (Variables|/Game/BistroBlitz/Blueprints/Holdables/BP_Holdable.BP_Holdable_C|GetID _array_element) (Variables|Default|GetHighestID))
      (Variables|Default|SetHighestID (Variables|/Game/BistroBlitz/Blueprints/Holdables/BP_Holdable.BP_Holdable_C|GetID _array_element))))
  (bind _holdable_reference (CallFunction|FindHoldable "/Game/BistroBlitz/Blueprints/Holdables/BP_Order.BP_Order_C" (Variables|Default|GetHighestID)))
  (bind _asbp_order (Utilities|Casting|CastToBP_Order _holdable_reference))
  (bind _order (Default|CreateRandomOrder _asbp_order))
  (Variables|Default|SetOrder _order)
  (Variables|Default|SetHasOrder true)
  (CallFunction|Hold (Variables|Default|GetHighestID) Character))

(event EventBeginPlay
  (|CallParentFunction) ; This node is disabled and will not be called.\nDrag off pins to build functionality.
)

(event Collision|EventActorBeginOverlap
  (params (OtherActor :type Actor%20Object%20Reference))
  (|CallParentFunction OtherActor) ; This node is disabled and will not be called.\nDrag off pins to build functionality.
)

(event EventTick
  (params (DeltaSeconds :type Float%20%28single-precision%29))
  (|CallParentFunction DeltaSeconds))

(fn ConstructionScript
  (|CallParentFunction))

(fn Interact
  (params (CurrentHoldable :type BP%20Holdable%20Object%20Reference) (CurrentPlayer :type BP%20Bistro%20Blitz%20Character%20Object%20Reference) (ItemIndex :type Integer) (HoldableType :type BP%20Holdable%20Class%20Reference))
  (LocalVariables|SetNewLocalVar CurrentPlayer)
  (bind _output_get (LocalVariables|SetNewLocalVar_0 ItemIndex))
  (bind _output_get_2 (LocalVariables|SetNewLocalVar_1 HoldableType))
  (bind _holdable_reference (CallFunction|FindHoldable _output_get_2 _output_get))
  (LocalVariables|SetNewLocalVar_2 _holdable_reference)
  (|CallParentFunction 0 0 0 0)
  (Actor|GetAllActorsOfClass "/Game/BistroBlitz/Blueprints/AI/BP_BistroBlitzCustomer.BP_BistroBlitzCustomer_C")
  (Utilities|IsValid (Variables|Default|GetCustomer)
    (:Is%20Valid
      (if (Variables|/Game/BistroBlitz/Blueprints/BP_BistroBlitzCharacter.BP_BistroBlitzCharacter_C|GetHolding (LocalVariables|GetNewLocalVar))
        ;[0.03646 0.03646 0.03646] Placing dish on table
        (bind _asbp_plate (Utilities|Casting|CastToBP_Plate (LocalVariables|GetNewLocalVar_2)))
        (if (Variables|Default|GetHasOrder)
          (CallFunction|RemoveClocheServer (LocalVariables|GetNewLocalVar_1) (LocalVariables|GetNewLocalVar_0))
          (Utilities|FlowControl|Sequence
            (:then_0
              ;;[0.03646 0.03646 0.03646] Rebuild the meshes for the dish
              (for _array_element (Variables|/Game/BistroBlitz/Blueprints/Holdables/BP_Plate.BP_Plate_C|GetHoldables _asbp_plate)
                (Utilities|Array|Add (LocalVariables|GetNewLocalVar_3) (Utilities|GetClass _array_element))
                (Utilities|Array|Add (LocalVariables|GetNewLocalVar_4) (Variables|/Game/BistroBlitz/Blueprints/Holdables/BP_Holdable.BP_Holdable_C|GetID _array_element)))
              (Default|SetHolding (LocalVariables|GetNewLocalVar) 0 "/Game/BistroBlitz/Blueprints/Holdables/BP_Nothing.BP_Nothing_C" 0 false)
              (CallFunction|CreateMeshesServer (LocalVariables|GetNewLocalVar_3) (LocalVariables|GetNewLocalVar_4)))
            (:then_1
              (Variables|Default|SetPlateNumber (LocalVariables|GetNewLocalVar_0)))
            (:then_2
              (AI|Components|Blackboard|SetValueasBool (Variables|/Script/AIModule.AIController|GetBlackboard (AI|GetAIController (Variables|Default|GetCustomer))) (Utilities|Name|MakeLiteralName "HasFood") true)
              (Variables|Default|SetHasFood true))))
        (elif (not (Variables|Default|GetHasOrder))
          (bind _aspc_bistro_blitz (Utilities|Casting|CastToPC_BistroBlitz (Game|GetPlayerController 0)))
          (Default|SpawnActorServer _aspc_bistro_blitz "/Game/BistroBlitz/Blueprints/Holdables/BP_Order.BP_Order_C" (Math|Transform|MakeTransform "1000.000000,0.000000,-50.000000"))
          (CallFunction|DoOrder (LocalVariables|GetNewLocalVar)))))
    (:Is%20Not%20Valid
      (Development|PrintString "it broke" true true "(R=0.000000,G=1.000000,B=0.361717,A=1.000000)" 86.0))))

(fn JudgeDish
  (bind _returnvalue (Utilities|Name|MakeLiteralName "Happiness"))
  (bind _order (Variables|Default|GetOrder))
  (bind _asgi_server_info (Utilities|Casting|CastToGI_ServerInfo (Game|GetGameInstance)))
  (LocalVariables|SetGameInstance _asgi_server_info)
  ;[0.03646 0.03646 0.03646] Do things lol
  (bind _holdable_reference (CallFunction|FindHoldable "/Game/BistroBlitz/Blueprints/Holdables/BP_Plate.BP_Plate_C" (Variables|Default|GetPlateNumber)))
  (bind _asbp_plate (Utilities|Casting|CastToBP_Plate _holdable_reference))
  (bind _food (Default|GetFood _asbp_plate))
  (LocalVariables|SetFood _food)
  (for (_array_element _array_index) _food
    (if (< _array_index (Utilities|Array|Length _order))
      ;;[1 1 1] If the item is in the correct order, give full points
      (if (== _array_element (Utilities|Array|Get(acopy) _order _array_index))
        (Math|Float|IncrementFloat (LocalVariables|GetScore)
          (:%20%20
            (Utilities|Array|RemoveItem (LocalVariables|GetFood) _array_element)))
        (else
          ;;[1 1 1] Give half points if the item is in the dish but in the wrong order
          (if (Utilities|Array|ContainsItem (LocalVariables|GetFood) (Utilities|Array|Get(acopy) _order _array_index))
            (LocalVariables|SetScore (+ (LocalVariables|GetScore) 0.5))
            (Utilities|Array|RemoveItem (LocalVariables|GetFood) _array_element))))))
  (for _array_element_2 (Variables|Default|GetOrder)
    (switch name _array_element_2
      (:Tomato-Sliced
        (LocalVariables|SetPrice (+ (LocalVariables|GetPrice) 0.2)))
      (:Tomato
        (LocalVariables|SetPrice (+ (LocalVariables|GetPrice) 0.5)))
      (:Bread
        (LocalVariables|SetPrice (+ (LocalVariables|GetPrice) 1.0)))
      (:Bread-Sliced
        (LocalVariables|SetPrice (+ (LocalVariables|GetPrice) 0.3)))
      (:Bottom-Bun
        (LocalVariables|SetPrice (+ (LocalVariables|GetPrice) 0.2)))
      (:Top-Bun
        (LocalVariables|SetPrice (+ (LocalVariables|GetPrice) 0.2)))
      (:Cheese
        (LocalVariables|SetPrice (+ (LocalVariables|GetPrice) 0.8)))
      (:Cheese-Sliced
        (LocalVariables|SetPrice (+ (LocalVariables|GetPrice) 0.2)))
      (:Egg
        (LocalVariables|SetPrice (+ (LocalVariables|GetPrice) 0.2)))
      (:Egg-Fried
        (LocalVariables|SetPrice (+ (LocalVariables|GetPrice) 0.35)))
      (:Raw-Beef
        (LocalVariables|SetPrice (+ (LocalVariables|GetPrice) 0.5)))
      (:Cooked-Patty
        (LocalVariables|SetPrice (+ (LocalVariables|GetPrice) 0.75)))
      (:Lettuce-Head
        (LocalVariables|SetPrice (+ (LocalVariables|GetPrice) 0.8)))
      (:Lettuce
        (LocalVariables|SetPrice (+ (LocalVariables|GetPrice) 0.15)))
      (:Mushtoom
        (LocalVariables|SetPrice (+ (LocalVariables|GetPrice) 0.4)))
      (:Mushroom-Slice
        (LocalVariables|SetPrice (+ (LocalVariables|GetPrice) 0.25)))
      (:Pan
        (LocalVariables|SetPrice (+ (LocalVariables|GetPrice) 2.0)))
      (:Plate
        (LocalVariables|SetPrice (+ (LocalVariables|GetPrice) 1.0)))))
  (Default|AddScore (LocalVariables|GetGameInstance) (/ (LocalVariables|GetScore) (Utilities|Array|Length (Variables|Default|GetOrder))) (+ (LocalVariables|GetPrice) 1.5))
  (bind _asbp_bbc_aicontroller (Utilities|Casting|CastToBP_BBC_AIController (AI|GetAIController (Variables|Default|GetCustomer))))
  (AI|Components|Blackboard|SetValueasFloat (AI|GetBlackboard _asbp_bbc_aicontroller) _returnvalue (Math|Float|Min(Float) (+ (Class|BlackboardComponent|GetValueasFloat (AI|GetBlackboard _asbp_bbc_aicontroller) _returnvalue) (Math|Float|Lerp -5e+01 2e+01 (/ (LocalVariables|GetScore) (Utilities|Array|Length (Variables|Default|GetOrder))))) 1e+02))
  (CallFunction|RemoveDishMulti))

(fn RemoveDish
  (for _array_element (Variables|Default|GetMeshes)
    (Components|DestroyComponent _array_element))
  (Utilities|Array|Clear (Variables|Default|GetMeshes))
  (Variables|Default|SetMeshes (Variables|Default|GetMeshes))
  (Utilities|Array|Clear (Variables|Default|GetOrder))
  (Variables|Default|SetOrder (Variables|Default|GetOrder))
  (Variables|Default|SetCustomer 0)
  (Variables|Default|SetHasCustomer false)
  (Variables|Default|SetHasOrder false)
  (Variables|Default|SetRef_Plate 0)
  (Components|StaticMesh|SetStaticMesh (Variables|Default|GetPlate) 0)
  (Variables|Default|SetLastTransform (Math|Transform|MakeTransform "-80.000000,0.000000,51.000000" "0, 0, 0" "0.350000,0.350000,0.350000")))

(fn GetInteractionInformation
  (params (HeldItem :type BP%20Holdable%20Object%20Reference))
  (bind (_canbecut _hasbeencut _canbecooked _hasbeencooked _isplate _ispan _isnothing _ismop _isorder _hasfood) (Default|GetObjectInformation HeldItem))
  (if (Variables|Default|GetHasCustomer)
    (if (Variables|Default|GetHasOrder)
      (if (and _isplate _hasfood)
        (LocalVariables|SetText "Serve dish")
        (elif _isnothing
          (LocalVariables|SetText "Bring a dish to customer")
          (else
            (LocalVariables|SetText "Customer can't eat that"))))
      (elif _isnothing
        (LocalVariables|SetText "Take order")
        (else
          (LocalVariables|SetText "Empty hands to take order"))))
    (else
      (LocalVariables|SetText "No customer is present")))
  (return (Utilities|Text|ToText(String) (LocalVariables|GetText)) true 1.0 false))