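; Mess spawner actor for Bistro Blitz that periodically drops BP_Mess actors inside its box volume.
; A tick counter, frame-rate dependent and noted as temporary, resets past a threshold and calls SpawnMessServer, which forwards to SpawnMessMulti.
; Each mess spawns at a random XY in the box at the spawner's height, with random yaw and scale.
; Spawning ignores collision, so messes can land under tables.
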(event Custom|SpawnMessServer
  (CallFunction|SpawnMessMulti))

(event Custom|SpawnMessMulti
  (bind _self self)
  (bind _box (Variables|Default|GetBox))
  (bind _returnvalue (Transformation|GetActorLocation _self))
  (bind _boxextent (Variables|/Script/Engine.BoxComponent|GetBoxExtent _box))
  (bind _returnvalue_2 (Math|Random|RandomPointinBoundingBox _returnvalue _boxextent))
  ;[1 1 1] this can currently spawn under tables
  (Game|SpawnActorfromClass "/Game/BistroBlitz/Blueprints/Stations/BP_Mess.BP_Mess_C" (Math|Transform|MakeTransform (Math|Vector|MakeVector (.x _returnvalue_2) (.y _returnvalue_2) (.z (.location (Transformation|GetActorTransform)))) (Math|Rotator|MakeRotator 0.0 0.0 (* (Math|Random|RandomFloat) 3.6e+02)) (Math|Conversions|ToVector(Float) (+ (* (Math|Random|RandomFloat) 0.3) 1.3))) "AlwaysSpawn" "MultiplyWithRoot" 0 0))

(event EventTick
  (params (DeltaSeconds :type Float%20%28single-precision%29))
  ;[1 1 1] this is temporary ill probably change it to each customer adds to the counter the angrier the more they add but that will probably be really  inefficient so idl if thats a great idea
  (bind _result (Math|Float|IncrementFloat (Variables|Default|Getcounter))
    (:%20%20
      (if (> _result 5e+02)
        (Variables|Default|Setcounter 0.0)
        (CallFunction|SpawnMessServer)))))

(fn ConstructionScript)