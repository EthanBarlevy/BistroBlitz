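; PC_MainMenu is the main menu player controller for BistroBlitz.
; On BeginPlay it caches the GI_ServerInfo game instance, then creates and shows the UI_MainMenu widget with the mouse cursor visible and UI-only input.
; Its ClientHostSession event forwards session hosting to the game instance's HostSession.
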(event Custom|Client%20Host%20Session
  (Default|HostSession (Variables|Default|GetRef_ServerInfo)))

(event EventBeginPlay
  (bind _asgi_server_info (Utilities|Casting|CastToGI_ServerInfo (Game|GetGameInstance)))
  (Variables|Default|SetRef_ServerInfo _asgi_server_info)
  (Utilities|IsValid (stale _returnvalue)
    (:Is%20Valid
      _)
    (:Is%20Not%20Valid
      (bind _returnvalue (UserInterface|CreateWidget "/Game/BistroBlitz/UI/UI_MainMenu.UI_MainMenu_C" (Game|GetPlayerController 0)))))
  (UserInterface|Viewport|AddtoViewport _returnvalue 0)
  (Variables|Default|SetbShowMouseCursor true)
  (Input|SetInputModeUIOnly (Game|GetPlayerController 0) _returnvalue "DoNotLock" false))

(fn ConstructionScript)