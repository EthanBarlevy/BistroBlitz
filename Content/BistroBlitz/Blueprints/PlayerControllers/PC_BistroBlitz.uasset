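; Bistro Blitz player controller that manages each player's HUD prompts, fridge and pause menus, and ready state.
; HUD events forward to BP_HUD only when their IsServer flag matches the machine's role, while SpawnActorServer numbers spawns by existing count.
; Fridge and pause widgets are created on demand and toggle input mode and cursor.
; Escape or debug Q calls GI_ServerInfo's Remove, then closes the open fridge or toggles pause; Ready/Unready also forward there.
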(event Custom|Ready
  (bind _asgi_server_info (Utilities|Casting|CastToGI_ServerInfo (Game|GetGameInstance)))
  (Default|Ready _asgi_server_info))

(event Custom|Add%20/%20Remove%20Fridge
  (Utilities|IsValid (Variables|Default|Getfridge)
    (:Is%20Valid
      (if (UserInterface|Viewport|IsinViewport (Variables|Default|Getfridge))
        (Widget|RemovefromParent (Variables|Default|Getfridge))
        (Input|SetInputModeGameOnly (Game|GetPlayerController 0) true)
        (Variables|Default|SetbShowMouseCursor false)
        (else
          (UserInterface|Viewport|AddtoViewport (stale _returnvalue) 0 :!label _label)
          (Input|SetInputModeGameandUI (Game|GetPlayerController 0) (Variables|Default|Getfridge) "DoNotLock" false true)
          (Variables|Default|SetbShowMouseCursor true))))
    (:Is%20Not%20Valid
      (bind _returnvalue (UserInterface|CreateWidget "/Game/BistroBlitz/UI/UI_Fridge.UI_Fridge_C" (Game|GetPlayerController 0)))
      (bind _output_get (Variables|Default|Setfridge _returnvalue))
      (goto _label))))

(event Custom|Unready
  (bind _asgi_server_info (Utilities|Casting|CastToGI_ServerInfo (Game|GetGameInstance)))
  (Default|Unready _asgi_server_info))

(event Custom|SetVisibilty
  (params (visibility :type ESlateVisibility%20Enum :default "Visible") (only%20ft :type Boolean) (IsServer :type Boolean))
  (if (== (Networking|IsServer) IsServer)
    (bind _asbp_hud (Utilities|Casting|CastToBP_HUD (HUD|GetHUD)))
    (Default|SetVisiblility (Variables|/Game/BistroBlitz/UI/BP_HUD.BP_HUD_C|GetHUD _asbp_hud) visibility only%20ft)))

(event Custom|ShowInteraction
  (params (flavortext :type Text) (SingleUse :type Boolean) (RadialAmount :type Float%20%28double-precision%29) (OnlyShowFlavortext :type Boolean) (IsServer :type Boolean))
  (if (== (Networking|IsServer) IsServer)
    (bind _asbp_hud (Utilities|Casting|CastToBP_HUD (HUD|GetHUD)))
    (Default|ShowInteraction (Variables|/Game/BistroBlitz/UI/BP_HUD.BP_HUD_C|GetHUD _asbp_hud) flavortext SingleUse RadialAmount OnlyShowFlavortext)))

(event Custom|SpawnActorServer
  (params (Class :type BP%20Holdable%20Class%20Reference) (SpawnTransform :type Transform))
  (bind _outactors (Actor|GetAllActorsOfClass Class))
  (bind _returnvalue (Game|SpawnActorfromClass Class SpawnTransform "Undefined" "MultiplyWithRoot" 0 0))
  (Variables|/Game/BistroBlitz/Blueprints/Holdables/BP_Holdable.BP_Holdable_C|SetID _returnvalue (Utilities|Array|Length _outactors)))

(event EventBeginPlay
  (Input|SetInputModeGameOnly (Game|GetPlayerController 0) false))

(event Input|KeyboardEvents|DebugKeyQ
  (params (Key :type Key%20Structure :default "None") (ActionValue :type Input%20Action%20Value%20Structure))
  (bind _fridge (Variables|Default|Getfridge))
  ;[0.03646 0.03646 0.03646] Pause Screen
  (:Pressed
    (bind _asgi_server_info (Utilities|Casting|CastToGI_ServerInfo (Game|GetGameInstance)))
    (Default|Remove _asgi_server_info)
    (Utilities|IsValid _fridge
      (:Is%20Valid
        (if (UserInterface|Viewport|IsinViewport _fridge)
          (Default|UndoAll _fridge)
          (Widget|RemovefromParent _fridge)
          (Input|SetInputModeGameOnly (Game|GetPlayerController 0) true)
          (Variables|Default|SetbShowMouseCursor false)
          (else
            (Utilities|IsValid (stale _returnvalue) :!label _label
              (:Is%20Valid
                (if (UserInterface|Viewport|IsinViewport (stale _returnvalue))
                  (Widget|RemovefromParent (stale _returnvalue))
                  (Input|SetInputModeGameOnly (Game|GetPlayerController 0) true)
                  (Variables|Default|SetbShowMouseCursor false)
                  (else
                    (UserInterface|Viewport|AddtoViewport (stale _returnvalue) 0 :!label _label_2)
                    (Input|SetInputModeUIOnly (Game|GetPlayerController 0) (stale _returnvalue) "DoNotLock" true)
                    (Variables|Default|SetbShowMouseCursor true))))
              (:Is%20Not%20Valid
                (bind _returnvalue (UserInterface|CreateWidget "/Game/BistroBlitz/UI/UI_PauseMenu.UI_PauseMenu_C" (Game|GetPlayerController 0)))
                (Variables|Default|SetNewVar _returnvalue)
                (goto _label_2))))))
      (:Is%20Not%20Valid
        (goto _label)))))

(event Input|KeyboardEvents|Escape
  (params (Key :type Key%20Structure :default "None"))
  (bind _fridge (Variables|Default|Getfridge))
  ;[0.03646 0.03646 0.03646] Pause Screen
  (:Pressed
    (bind _asgi_server_info (Utilities|Casting|CastToGI_ServerInfo (Game|GetGameInstance)))
    (Default|Remove _asgi_server_info)
    (Utilities|IsValid _fridge
      (:Is%20Valid
        (if (UserInterface|Viewport|IsinViewport _fridge)
          (Default|UndoAll _fridge)
          (Widget|RemovefromParent _fridge)
          (Input|SetInputModeGameOnly (Game|GetPlayerController 0) true)
          (Variables|Default|SetbShowMouseCursor false)
          (else
            (Utilities|IsValid (stale _returnvalue) :!label _label
              (:Is%20Valid
                (if (UserInterface|Viewport|IsinViewport (stale _returnvalue))
                  (Widget|RemovefromParent (stale _returnvalue))
                  (Input|SetInputModeGameOnly (Game|GetPlayerController 0) true)
                  (Variables|Default|SetbShowMouseCursor false)
                  (else
                    (UserInterface|Viewport|AddtoViewport (stale _returnvalue) 0 :!label _label_2)
                    (Input|SetInputModeUIOnly (Game|GetPlayerController 0) (stale _returnvalue) "DoNotLock" true)
                    (Variables|Default|SetbShowMouseCursor true))))
              (:Is%20Not%20Valid
                (bind _returnvalue (UserInterface|CreateWidget "/Game/BistroBlitz/UI/UI_PauseMenu.UI_PauseMenu_C" (Game|GetPlayerController 0)))
                (Variables|Default|SetNewVar _returnvalue)
                (goto _label_2))))))
      (:Is%20Not%20Valid
        (goto _label)))))

(fn ConstructionScript
  (|CallParentFunction))