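; AI customer for Bistro Blitz that takes a seat, shows its mood and can leave messes.
; Blackboard Happiness starts full and each tick tints both dynamic materials from red to green.
; While seated, a per-tick random roll asks GI_ServerInfo to spawn mess, likelier as happiness drops.
; SetTableSlot writes table and exit locations to the blackboard; SitAtTable teleports it to its ChairID slot and swaps to the sitting mesh.
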(event Custom|sitplease
  (bind _returnvalue (Transformation|GetActorTransform))
  (bind _sit_transform (Variables|Default|GetSit%20Transform))
  (bind _asbp_bbc_aicontroller (Utilities|Casting|CastToBP_BBC_AIController (AI|GetAIController self)))
  (AI|Navigation|StopMovement _asbp_bbc_aicontroller)
  (if (Variables|Default|GetSitting)
    (if (or (Utilities|Operators|NotEqual(!=) (.rotation _returnvalue) (.rotation _sit_transform) 0.5) (Utilities|Operators|NotEqual(!=) (.location _returnvalue) (.location _sit_transform) 1.0))
      (Transformation|SetActorTransform (Variables|Default|GetSit%20Transform) false true))))

(event Custom|sit
  (CallFunction|SitatTable))

(event Custom|sit%20server
  (CallFunction|Sit))

(event Custom|ChangeColor%20Server
  (CallFunction|ChangeColor))

(event Custom|Change%20Color
  (bind _self self)
  (bind _color_material1 (Variables|Default|GetColor%20Material1))
  (bind _color_material2 (Variables|Default|GetColor%20Material2))
  (Utilities|IsValid _self
    (:Is%20Valid
      (bind _asbp_bbc_aicontroller (Utilities|Casting|CastToBP_BBC_AIController (AI|GetAIController _self)))
      (Utilities|IsValid _color_material1
        (:Is%20Valid
          (Rendering|Material|SetVectorParameterValue _color_material1 "Base Color" (Math|Color|Lerp(LinearColor) (Math|Color|MakeColor 1.0 0.0 0.0) (Math|Color|MakeColor 0.0 1.0 0.0) (/ (Class|BlackboardComponent|GetValueasFloat (Variables|/Script/AIModule.AIController|GetBlackboard _asbp_bbc_aicontroller) (Utilities|Name|MakeLiteralName "Happiness")) 1e+02)) :!class /Script/Engine.MaterialInstanceDynamic)
          (Utilities|IsValid _color_material2
            (:Is%20Valid
              (Rendering|Material|SetVectorParameterValue _color_material2 "Base Color" (Math|Color|Lerp(LinearColor) (Math|Color|MakeColor 1.0 0.0 0.0) (Math|Color|MakeColor 0.0 1.0 0.0) (/ (Class|BlackboardComponent|GetValueasFloat (Variables|/Script/AIModule.AIController|GetBlackboard _asbp_bbc_aicontroller) (Utilities|Name|MakeLiteralName "Happiness")) 1e+02)) :!class /Script/Engine.MaterialInstanceDynamic))))))))

(event Custom|TrySpawnMess
  (bind _self self)
  (bind _asgi_server_info (Utilities|Casting|CastToGI_ServerInfo (Game|GetGameInstance)))
  (Utilities|IsValid _self
    (:Is%20Valid
      (bind _asbp_bbc_aicontroller (Utilities|Casting|CastToBP_BBC_AIController (AI|GetAIController _self)))
      (if (and (< (Math|Random|RandomFloatinRange -0.5 (Class|BlackboardComponent|GetValueasFloat (Variables|/Script/AIModule.AIController|GetBlackboard _asbp_bbc_aicontroller) (Utilities|Name|MakeLiteralName "Happiness"))) 0.0) (Variables|Default|GetSitting))
        (Default|TrySpawnMess _asgi_server_info)))))

(event EventBeginPlay
  (bind _mesh (Variables|Character|GetMesh))
  (bind _sittingmesh (Variables|Default|GetSittingMesh))
  (bind _returnvalue (Rendering|Material|CreateDynamicMaterialInstance _mesh 0 "/Game/BistroBlitz/Materials/M_Yellow.M_Yellow" "None" :!class /Script/Engine.PrimitiveComponent))
  (bind _output_get (Variables|Default|SetColor%20Material1 _returnvalue))
  (Rendering|Material|SetMaterial _mesh 0 _output_get)
  (bind _returnvalue_2 (Rendering|Material|CreateDynamicMaterialInstance _sittingmesh 0 "/Game/BistroBlitz/Materials/M_Yellow.M_Yellow" "None" :!class /Script/Engine.PrimitiveComponent))
  (bind _output_get_2 (Variables|Default|SetColor%20Material2 _returnvalue_2))
  (Rendering|Material|SetMaterial _sittingmesh 0 _output_get_2)
  (bind _asbp_bbc_aicontroller (Utilities|Casting|CastToBP_BBC_AIController (AI|GetAIController self)))
  (AI|Components|Blackboard|SetValueasFloat (Variables|/Script/AIModule.AIController|GetBlackboard _asbp_bbc_aicontroller) (Utilities|Name|MakeLiteralName "Happiness") 1e+02))

(event EventTick
  (params (DeltaSeconds :type Float%20%28single-precision%29))
  (CallFunction|ChangeColorServer)
  (CallFunction|TrySpawnMess))

(fn ConstructionScript)

(fn SetTableSlot
  (params (Location :type Integer) (Exit :type BP%20Customer%20Exit%20Object%20Reference))
  (Development|PrintString (Utilities|String|ToString(Integer) (Variables|Default|GetID)) true true "(R=1.000000,G=0.433272,B=0.594815,A=1.000000)" 1e+01)
  (Development|PrintString (Utilities|String|ToString(Integer) (Variables|Default|GetChairID)) true true "(R=0.459838,G=1.000000,B=0.545567,A=1.000000)" 1e+01)
  (Development|PrintString (Utilities|String|ToString(Integer) Location))
  (bind _asbp_bbc_aicontroller (Utilities|Casting|CastToBP_BBC_AIController (AI|GetAIController self)))
  (bind _outactors (Actor|GetAllActorsOfClass "/Game/BistroBlitz/Blueprints/Stations/BP_TableSlot.BP_TableSlot_C"))
  (for _array_element _outactors
    (if (== (Variables|/Game/BistroBlitz/Blueprints/Stations/BP_TableSlot.BP_TableSlot_C|GetSeatNumber _array_element) Location)
      (LocalVariables|SetNewLocalVar _array_element)))
  (Utilities|FlowControl|Sequence
    (:then_0
      (AI|Components|Blackboard|SetValueasVector (Variables|/Script/AIModule.AIController|GetBlackboard _asbp_bbc_aicontroller) (Utilities|Name|MakeLiteralName "Table") (Transformation|GetActorLocation (LocalVariables|GetNewLocalVar))))
    (:then_1
      (AI|Components|Blackboard|SetValueasVector (Variables|/Script/AIModule.AIController|GetBlackboard _asbp_bbc_aicontroller) (Utilities|Name|MakeLiteralName "ExitPoint") (Transformation|GetActorLocation Exit)))))

(fn SitatTable
  (bind _outactors (Actor|GetAllActorsOfClass "/Game/BistroBlitz/Blueprints/Stations/BP_TableSlot.BP_TableSlot_C"))
  (for _array_element _outactors
    (if (== (Variables|/Game/BistroBlitz/Blueprints/Stations/BP_TableSlot.BP_TableSlot_C|GetSeatNumber _array_element) (Variables|Default|GetChairID))
      (LocalVariables|SetChair _array_element)))
  (bind _output_get (Variables|Default|SetSit%20Transform (Variables|/Game/BistroBlitz/Blueprints/Stations/BP_TableSlot.BP_TableSlot_C|GetSitTransform (LocalVariables|GetChair))))
  (Transformation|SetActorTransform self _output_get false true)
  (Variables|Default|SetSitting true)
  (Rendering|SetVisibility (Variables|Character|GetMesh) false false)
  (Rendering|SetVisibility (Variables|Default|GetSittingMesh) true false)
  (CallFunction|Sitplease))