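; Behavior tree task that makes a Bistro Blitz customer give up its seat, as an angry leave by its name.
; It searches all BP_TableSlot actors for the seat number matching the customer's ChairID and removes that table number from the table records in GI_ServerInfo.
; It then clears the Sitting flag, swaps which of the customer's two meshes is visible and finishes successfully.
; No failure finish is called if no seat matches or a cast fails.
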(event EventReceiveExecuteAI
  (params (OwnerController :type AI%20Controller%20Object%20Reference) (ControlledPawn :type Pawn%20Object%20Reference))
  (bind _asbp_bistro_blitz_customer (Utilities|Casting|CastToBP_BistroBlitzCustomer ControlledPawn))
  (bind _outactors (Actor|GetAllActorsOfClass "/Game/BistroBlitz/Blueprints/Stations/BP_TableSlot.BP_TableSlot_C"))
  (for _array_element _outactors
    (if (== (Variables|/Game/BistroBlitz/Blueprints/Stations/BP_TableSlot.BP_TableSlot_C|GetSeatNumber _array_element) (Variables|/Game/BistroBlitz/Blueprints/AI/BP_BistroBlitzCustomer.BP_BistroBlitzCustomer_C|GetChairID _asbp_bistro_blitz_customer))
      (bind _asgi_server_info (Utilities|Casting|CastToGI_ServerInfo (Game|GetGameInstance)))
      (Default|RemovefromTable _asgi_server_info (Variables|/Game/BistroBlitz/Blueprints/Stations/BP_TableSlot.BP_TableSlot_C|GetTableNumber _array_element))
      (Variables|/Game/BistroBlitz/Blueprints/AI/BP_BistroBlitzCustomer.BP_BistroBlitzCustomer_C|SetSitting _asbp_bistro_blitz_customer false)
      (Variables|/Game/BistroBlitz/Blueprints/AI/BP_BistroBlitzCustomer.BP_BistroBlitzCustomer_C|SetMeshVisible _asbp_bistro_blitz_customer true)
      (Variables|/Game/BistroBlitz/Blueprints/AI/BP_BistroBlitzCustomer.BP_BistroBlitzCustomer_C|SetMesh1Visible _asbp_bistro_blitz_customer false)
      (AI|BehaviorTree|FinishExecute true))))