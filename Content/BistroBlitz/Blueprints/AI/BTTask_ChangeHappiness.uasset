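; Behavior tree task that updates a Bistro Blitz customer's Happiness blackboard value on the customer's AI controller.
; It scans all BP_Mess actors and raises a multiplier from its base for each one within a fixed radius of the customer.
; Happiness is decremented, then scaled by that multiplier, so nearby messes enlarge the resulting value's magnitude.
; The task then finishes successfully, but a failed cast stops it without finishing.
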(event EventReceiveExecuteAI
  (params (OwnerController :type AI%20Controller%20Object%20Reference) (ControlledPawn :type Pawn%20Object%20Reference))
  (bind _returnvalue (Utilities|Name|MakeLiteralName "Happiness"))
  (bind _asbp_bistro_blitz_customer (Utilities|Casting|CastToBP_BistroBlitzCustomer ControlledPawn))
  (Variables|Default|Setmultiplier 1.0)
  (bind _asbp_bbc_aicontroller (Utilities|Casting|CastToBP_BBC_AIController (AI|GetAIController _asbp_bistro_blitz_customer)))
  (bind _outactors (Actor|GetAllActorsOfClass "/Game/BistroBlitz/Blueprints/Stations/BP_Mess.BP_Mess_C"))
  (for _array_element _outactors
    (if (< (Math|Vector|VectorLength (- (.location (Transformation|GetActorTransform _asbp_bistro_blitz_customer)) (.location (Transformation|GetActorTransform _array_element)))) 5e+02)
      (Variables|Default|Setmultiplier (+ (Variables|Default|Getmultiplier) 0.1))))
  (AI|Components|Blackboard|SetValueasFloat (Variables|/Script/AIModule.AIController|GetBlackboard _asbp_bbc_aicontroller) _returnvalue (* (- (Class|BlackboardComponent|GetValueasFloat (Variables|/Script/AIModule.AIController|GetBlackboard _asbp_bbc_aicontroller) _returnvalue) 1.0) (Variables|Default|Getmultiplier)))
  (AI|BehaviorTree|FinishExecute true))