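; Behavior tree task for Bistro Blitz customer AI that checks whether every ordered slot at the customer's table has food.
; It scans all BP_TableSlot actors for those matching the TableNumber blackboard value, ignoring slots without orders.
; The task finishes with the Everyone flag as its result, stopping the scan with failure at the first ordered slot still lacking food.
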(event EventReceiveExecuteAI
  (params (OwnerController :type AI%20Controller%20Object%20Reference) (ControlledPawn :type Pawn%20Object%20Reference))
  (bind _asbp_bistro_blitz_customer (Utilities|Casting|CastToBP_BistroBlitzCustomer ControlledPawn))
  (bind _outactors (Actor|GetAllActorsOfClass "/Game/BistroBlitz/Blueprints/Stations/BP_TableSlot.BP_TableSlot_C"))
  (bind _array_element (Utilities|Array|ForEachLoopwithBreak _outactors :!label _label)
    (:LoopBody
      (if (== (Variables|/Game/BistroBlitz/Blueprints/Stations/BP_TableSlot.BP_TableSlot_C|GetTableNumber _array_element) (Class|BlackboardComponent|GetValueasInt (AI|GetBlackboard (AI|GetAIController _asbp_bistro_blitz_customer)) (Utilities|Name|MakeLiteralName "TableNumber")))
        (if (Variables|/Game/BistroBlitz/Blueprints/Stations/BP_TableSlot.BP_TableSlot_C|GetHasOrder _array_element)
          (if (Variables|/Game/BistroBlitz/Blueprints/Stations/BP_TableSlot.BP_TableSlot_C|GetHasFood _array_element)
            (Variables|Default|Seteveryone true)
            (else
              (Variables|Default|Seteveryone false)
              (goto _label Break))))))
    (:Completed
      (AI|BehaviorTree|FinishExecute (Variables|Default|Geteveryone)))))