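; Fridge interior render actor that displays stocked ingredients and saucepans and highlights them by item type.
; On BeginPlay its SceneCaptureComponent2D is restricted to show only this actor and its child actors.
; Hover swaps every mesh of the given item type to M_Selected.
; UnHover restores each mesh's hardcoded original material, either for one type or for all types at once.
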(event EventBeginPlay
  (Rendering|SceneCapture|ShowOnlyActorComponents (Variables|Default|GetSceneCaptureComponent2D) self true))

(fn ConstructionScript)

(fn Hover
  (params (ItemType :type E_Food%20Enum :default "NewEnumerator0"))
  (bind _tomato (Variables|Default|Gettomato))
  (bind _tomato1 (Variables|Default|Gettomato1))
  (bind _bread (Variables|Default|GetBread))
  (bind _bread1 (Variables|Default|GetBread1))
  (bind _tomato2 (Variables|Default|Gettomato2))
  (switch Utilities|FlowControl|Switch|SwitchonE_Food ItemType
    (:NewEnumerator0
      (Utilities|FlowControl|Sequence
        (:then_0
          (Rendering|Material|SetMaterial _tomato 0 "/Game/BistroBlitz/Materials/M_Selected.M_Selected")
          (Rendering|Material|SetMaterial _tomato 1 "/Game/BistroBlitz/Materials/M_Selected.M_Selected"))
        (:then_1
          (Rendering|Material|SetMaterial _tomato1 0 "/Game/BistroBlitz/Materials/M_Selected.M_Selected")
          (Rendering|Material|SetMaterial _tomato1 1 "/Game/BistroBlitz/Materials/M_Selected.M_Selected"))
        (:then_2
          (Rendering|Material|SetMaterial _tomato2 0 "/Game/BistroBlitz/Materials/M_Selected.M_Selected")
          (Rendering|Material|SetMaterial _tomato2 1 "/Game/BistroBlitz/Materials/M_Selected.M_Selected"))))
    (:NewEnumerator1
      (Rendering|Material|SetMaterial (Variables|Default|Getbeef) 0 "/Game/BistroBlitz/Materials/M_Selected.M_Selected"))
    (:NewEnumerator2
      (Utilities|FlowControl|Sequence
        (:then_0
          (Rendering|Material|SetMaterial (Variables|Default|Getcheese) 0 "/Game/BistroBlitz/Materials/M_Selected.M_Selected"))
        (:then_1
          (Rendering|Material|SetMaterial (Variables|Default|Getcheese1) 0 "/Game/BistroBlitz/Materials/M_Selected.M_Selected"))))
    (:NewEnumerator3
      (Utilities|FlowControl|Sequence
        (:then_0
          (Rendering|Material|SetMaterial (Variables|Default|Getlettuce4) 0 "/Game/BistroBlitz/Materials/M_Selected.M_Selected"))
        (:then_1
          (Rendering|Material|SetMaterial (Variables|Default|Getlettuce5) 0 "/Game/BistroBlitz/Materials/M_Selected.M_Selected"))))
    (:NewEnumerator4
      (Utilities|FlowControl|Sequence
        (:then_0
          (Rendering|Material|SetMaterial (Variables|Default|GetmushroomWhole) 0 "/Game/BistroBlitz/Materials/M_Selected.M_Selected"))
        (:then_1
          (Rendering|Material|SetMaterial (Variables|Default|GetmushroomWhole3) 0 "/Game/BistroBlitz/Materials/M_Selected.M_Selected"))
        (:then_2
          (Rendering|Material|SetMaterial (Variables|Default|GetmushroomWhole2) 0 "/Game/BistroBlitz/Materials/M_Selected.M_Selected"))
        (:then_3
          (Rendering|Material|SetMaterial (Variables|Default|GetmushroomWhole1) 0 "/Game/BistroBlitz/Materials/M_Selected.M_Selected"))))
    (:NewEnumerator5
      (Utilities|FlowControl|Sequence
        (:then_0
          (Rendering|Material|SetMaterial (Variables|Default|Getpan2) 0 "/Game/BistroBlitz/Materials/M_Selected.M_Selected"))
        (:then_1
          (Rendering|Material|SetMaterial (Variables|Default|Getpan3) 0 "/Game/BistroBlitz/Materials/M_Selected.M_Selected"))))
    (:NewEnumerator6
      (Utilities|FlowControl|Sequence
        (:then_0
          (Rendering|Material|SetMaterial _bread 0 "/Game/BistroBlitz/Materials/M_Selected.M_Selected")
          (Rendering|Material|SetMaterial _bread 1 "/Game/BistroBlitz/Materials/M_Selected.M_Selected"))
        (:then_1
          (Rendering|Material|SetMaterial _bread1 0 "/Game/BistroBlitz/Materials/M_Selected.M_Selected")
          (Rendering|Material|SetMaterial _bread1 1 "/Game/BistroBlitz/Materials/M_Selected.M_Selected"))))
    (:NewEnumerator7
      (Utilities|FlowControl|Sequence
        (:then_0
          (Rendering|Material|SetMaterial (Variables|Default|Getbuntop) 0 "/Game/BistroBlitz/Materials/M_Selected.M_Selected"))
        (:then_1
          (Rendering|Material|SetMaterial (Variables|Default|Getbuntop1) 0 "/Game/BistroBlitz/Materials/M_Selected.M_Selected"))
        (:then_2
          (Rendering|Material|SetMaterial (Variables|Default|Getbuntop3) 0 "/Game/BistroBlitz/Materials/M_Selected.M_Selected"))
        (:then_3
          (Rendering|Material|SetMaterial (Variables|Default|Getbuntop5) 0 "/Game/BistroBlitz/Materials/M_Selected.M_Selected"))
        (:then_4
          (Rendering|Material|SetMaterial (Variables|Default|Getbuntop4) 0 "/Game/BistroBlitz/Materials/M_Selected.M_Selected"))
        (:then_5
          (Rendering|Material|SetMaterial (Variables|Default|Getbuntop2) 0 "/Game/BistroBlitz/Materials/M_Selected.M_Selected"))))
    (:NewEnumerator8
      (Utilities|FlowControl|Sequence
        (:then_0
          (Rendering|Material|SetMaterial (Variables|Default|Getbun-bottom) 0 "/Game/BistroBlitz/Materials/M_Selected.M_Selected"))
        (:then_1
          (Rendering|Material|SetMaterial (Variables|Default|Getbun-bottom1) 0 "/Game/BistroBlitz/Materials/M_Selected.M_Selected"))
        (:then_2
          (Rendering|Material|SetMaterial (Variables|Default|Getbun-bottom2) 0 "/Game/BistroBlitz/Materials/M_Selected.M_Selected"))
        (:then_3
          (Rendering|Material|SetMaterial (Variables|Default|Getbun-bottom6) 0 "/Game/BistroBlitz/Materials/M_Selected.M_Selected"))
        (:then_4
          (Rendering|Material|SetMaterial (Variables|Default|Getbun-bottom5) 0 "/Game/BistroBlitz/Materials/M_Selected.M_Selected"))
        (:then_5
          (Rendering|Material|SetMaterial (Variables|Default|Getbun-bottom7) 0 "/Game/BistroBlitz/Materials/M_Selected.M_Selected"))
        (:then_6
          (Rendering|Material|SetMaterial (Variables|Default|Getbun-bottom4) 0 "/Game/BistroBlitz/Materials/M_Selected.M_Selected"))
        (:then_7
          (Rendering|Material|SetMaterial (Variables|Default|Getbun-bottom3) 0 "/Game/BistroBlitz/Materials/M_Selected.M_Selected"))))
    (:NewEnumerator9
      (Utilities|FlowControl|Sequence
        (:then_0
          (Rendering|Material|SetMaterial (Variables|Default|GetEgg_Whole) 0 "/Game/BistroBlitz/Materials/M_Selected.M_Selected"))
        (:then_1
          (Rendering|Material|SetMaterial (Variables|Default|GetEgg_Whole7) 0 "/Game/BistroBlitz/Materials/M_Selected.M_Selected"))
        (:then_2
          (Rendering|Material|SetMaterial (Variables|Default|GetEgg_Whole4) 0 "/Game/BistroBlitz/Materials/M_Selected.M_Selected"))
        (:then_3
          (Rendering|Material|SetMaterial (Variables|Default|GetEgg_Whole8) 0 "/Game/BistroBlitz/Materials/M_Selected.M_Selected"))
        (:then_4
          (Rendering|Material|SetMaterial (Variables|Default|GetEgg_Whole1) 0 "/Game/BistroBlitz/Materials/M_Selected.M_Selected"))
        (:then_5
          (Rendering|Material|SetMaterial (Variables|Default|GetEgg_Whole9) 0 "/Game/BistroBlitz/Materials/M_Selected.M_Selected"))))))

(fn UnHover
  (params (ItemType :type E_Food%20Enum :default "NewEnumerator0") (All :type Boolean))
  (bind _tomato (Variables|Default|Gettomato))
  (bind _tomato1 (Variables|Default|Gettomato1))
  (bind _bread (Variables|Default|GetBread))
  (bind _bread1 (Variables|Default|GetBread1))
  (bind _tomato2 (Variables|Default|Gettomato2))
  (if All
    (Utilities|FlowControl|Sequence
      (:then_0
        (Utilities|FlowControl|Sequence :!label _label
          (:then_0
            (Rendering|Material|SetMaterial _tomato 0 "/Game/BistroBlitz/Materials/M_Tomato_Red.M_Tomato_Red")
            (Rendering|Material|SetMaterial _tomato 1 "/Game/BistroBlitz/Materials/M_Tomato_Stem.M_Tomato_Stem"))
          (:then_1
            (Rendering|Material|SetMaterial _tomato1 0 "/Game/BistroBlitz/Materials/M_Tomato_Red.M_Tomato_Red")
            (Rendering|Material|SetMaterial _tomato1 1 "/Game/BistroBlitz/Materials/M_Tomato_Stem.M_Tomato_Stem"))
          (:then_2
            (Rendering|Material|SetMaterial _tomato2 0 "/Game/BistroBlitz/Materials/M_Tomato_Red.M_Tomato_Red")
            (Rendering|Material|SetMaterial _tomato2 1 "/Game/BistroBlitz/Materials/M_Tomato_Stem.M_Tomato_Stem"))))
      (:then_1
        (Rendering|Material|SetMaterial (Variables|Default|Getbeef) 0 "/Game/BistroBlitz/Materials/M_GroundBeef.M_GroundBeef" :!label _label_2))
      (:then_2
        (Utilities|FlowControl|Sequence :!label _label_3
          (:then_0
            (Rendering|Material|SetMaterial (Variables|Default|Getcheese) 0 "/Game/BistroBlitz/Materials/M_Cheese.M_Cheese"))
          (:then_1
            (Rendering|Material|SetMaterial (Variables|Default|Getcheese1) 0 "/Game/BistroBlitz/Materials/M_Cheese.M_Cheese"))))
      (:then_3
        (Utilities|FlowControl|Sequence :!label _label_4
          (:then_0
            (Rendering|Material|SetMaterial (Variables|Default|Getlettuce4) 0 "/Game/BistroBlitz/Materials/M_Lettuce.M_Lettuce"))
          (:then_1
            (Rendering|Material|SetMaterial (Variables|Default|Getlettuce5) 0 "/Game/BistroBlitz/Materials/M_Lettuce.M_Lettuce"))))
      (:then_4
        (Utilities|FlowControl|Sequence :!label _label_5
          (:then_0
            (Rendering|Material|SetMaterial (Variables|Default|GetmushroomWhole) 0 "/Game/BistroBlitz/Materials/M_MushroomExterior.M_MushroomExterior"))
          (:then_1
            (Rendering|Material|SetMaterial (Variables|Default|GetmushroomWhole3) 0 "/Game/BistroBlitz/Materials/M_MushroomExterior.M_MushroomExterior"))
          (:then_2
            (Rendering|Material|SetMaterial (Variables|Default|GetmushroomWhole2) 0 "/Game/BistroBlitz/Materials/M_MushroomExterior.M_MushroomExterior"))
          (:then_3
            (Rendering|Material|SetMaterial (Variables|Default|GetmushroomWhole1) 0 "/Game/BistroBlitz/Materials/M_MushroomExterior.M_MushroomExterior"))))
      (:then_5
        (Utilities|FlowControl|Sequence :!label _label_6
          (:then_0
            (Rendering|Material|SetMaterial (Variables|Default|Getpan2) 0 "/Game/BistroBlitz/Materials/M_Cloche.M_Cloche"))
          (:then_1
            (Rendering|Material|SetMaterial (Variables|Default|Getpan3) 0 "/Game/BistroBlitz/Materials/M_Cloche.M_Cloche"))))
      (:then_6
        (Utilities|FlowControl|Sequence :!label _label_7
          (:then_0
            (Rendering|Material|SetMaterial _bread 0 "/Game/BistroBlitz/Materials/M_BreadCrust.M_BreadCrust")
            (Rendering|Material|SetMaterial _bread 1 "/Game/BistroBlitz/Materials/M_Bread.M_Bread"))
          (:then_1
            (Rendering|Material|SetMaterial _bread1 0 "/Game/BistroBlitz/Materials/M_BreadCrust.M_BreadCrust")
            (Rendering|Material|SetMaterial _bread1 1 "/Game/BistroBlitz/Materials/M_Bread.M_Bread"))))
      (:then_7
        (Utilities|FlowControl|Sequence :!label _label_8
          (:then_0
            (Rendering|Material|SetMaterial (Variables|Default|Getbuntop) 0 "/Game/BistroBlitz/Materials/M_Bun.M_Bun"))
          (:then_1
            (Rendering|Material|SetMaterial (Variables|Default|Getbuntop1) 0 "/Game/BistroBlitz/Materials/M_Bun.M_Bun"))
          (:then_2
            (Rendering|Material|SetMaterial (Variables|Default|Getbuntop3) 0 "/Game/BistroBlitz/Materials/M_Bun.M_Bun"))
          (:then_3
            (Rendering|Material|SetMaterial (Variables|Default|Getbuntop5) 0 "/Game/BistroBlitz/Materials/M_Bun.M_Bun"))
          (:then_4
            (Rendering|Material|SetMaterial (Variables|Default|Getbuntop4) 0 "/Game/BistroBlitz/Materials/M_Bun.M_Bun"))
          (:then_5
            (Rendering|Material|SetMaterial (Variables|Default|Getbuntop2) 0 "/Game/BistroBlitz/Materials/M_Bun.M_Bun"))))
      (:then_8
        (Utilities|FlowControl|Sequence :!label _label_9
          (:then_0
            (Rendering|Material|SetMaterial (Variables|Default|Getbun-bottom) 0 "/Game/BistroBlitz/Materials/M_Bun.M_Bun"))
          (:then_1
            (Rendering|Material|SetMaterial (Variables|Default|Getbun-bottom1) 0 "/Game/BistroBlitz/Materials/M_Bun.M_Bun"))
          (:then_2
            (Rendering|Material|SetMaterial (Variables|Default|Getbun-bottom2) 0 "/Game/BistroBlitz/Materials/M_Bun.M_Bun"))
          (:then_3
            (Rendering|Material|SetMaterial (Variables|Default|Getbun-bottom6) 0 "/Game/BistroBlitz/Materials/M_Bun.M_Bun"))
          (:then_4
            (Rendering|Material|SetMaterial (Variables|Default|Getbun-bottom5) 0 "/Game/BistroBlitz/Materials/M_Bun.M_Bun"))
          (:then_5
            (Rendering|Material|SetMaterial (Variables|Default|Getbun-bottom7) 0 "/Game/BistroBlitz/Materials/M_Bun.M_Bun"))
          (:then_6
            (Rendering|Material|SetMaterial (Variables|Default|Getbun-bottom4) 0 "/Game/BistroBlitz/Materials/M_Bun.M_Bun"))
          (:then_7
            (Rendering|Material|SetMaterial (Variables|Default|Getbun-bottom3) 0 "/Game/BistroBlitz/Materials/M_Bun.M_Bun"))))
      (:then_9
        (Utilities|FlowControl|Sequence :!label _label_10
          (:then_0
            (Rendering|Material|SetMaterial (Variables|Default|GetEgg_Whole) 0 "/Game/BistroBlitz/Materials/M_EggWhite.M_EggWhite"))
          (:then_1
            (Rendering|Material|SetMaterial (Variables|Default|GetEgg_Whole7) 0 "/Game/BistroBlitz/Materials/M_EggWhite.M_EggWhite"))
          (:then_2
            (Rendering|Material|SetMaterial (Variables|Default|GetEgg_Whole4) 0 "/Game/BistroBlitz/Materials/M_EggWhite.M_EggWhite"))
          (:then_3
            (Rendering|Material|SetMaterial (Variables|Default|GetEgg_Whole8) 0 "/Game/BistroBlitz/Materials/M_EggWhite.M_EggWhite"))
          (:then_4
            (Rendering|Material|SetMaterial (Variables|Default|GetEgg_Whole1) 0 "/Game/BistroBlitz/Materials/M_EggWhite.M_EggWhite"))
          (:then_5
            (Rendering|Material|SetMaterial (Variables|Default|GetEgg_Whole9) 0 "/Game/BistroBlitz/Materials/M_EggWhite.M_EggWhite")))))
    (else
      (switch Utilities|FlowControl|Switch|SwitchonE_Food ItemType
        (:NewEnumerator0
          (goto _label))
        (:NewEnumerator1
          (goto _label_2))
        (:NewEnumerator2
          (goto _label_3))
        (:NewEnumerator3
          (goto _label_4))
        (:NewEnumerator4
          (goto _label_5))
        (:NewEnumerator5
          (goto _label_6))
        (:NewEnumerator6
          (goto _label_7))
        (:NewEnumerator7
          (goto _label_8))
        (:NewEnumerator8
          (goto _label_9))
        (:NewEnumerator9
          (goto _label_10))))))