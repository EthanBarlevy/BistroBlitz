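; Render actor for the sink station, showing an animated mesh through a scene capture.
; On BeginPlay, the SceneCaptureComponent2D is limited to this actor's own components and its child actors.
; Hover starts a Timeline that rotates the mesh in pitch and yaw, alternating forward and reverse playback.
; Unhover sets a stop flag, so the mesh resets to zero rotation once the current sweep finishes.
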(event Custom|hover
  (Variables|Default|Setstopped false)
  (bind _rotation (Timeline|Timeline PlayFromStart)
    (:Update
      (Transformation|SetRelativeRotation (Variables|Default|GetStaticMesh) (Math|Rotator|MakeRotator 0.0 _rotation _rotation) false false))
    (:Finished
      (bind _output_get (Variables|Default|Setstate (not (Variables|Default|Getstate))))
      (if _output_get
        (if (not (Variables|Default|Getstopped))
          (Timeline|Timeline Reverse)
          (else
            (Transformation|SetRelativeRotation (Variables|Default|GetStaticMesh) (Math|Rotator|MakeRotator 0.0 0.0 0.0) false false :!label _label)))
        (elif (not (Variables|Default|Getstopped))
          (Timeline|Timeline Play)
          (else
            (goto _label)))))))

(event Custom|unhover
  (Variables|Default|Setstopped true))

(event EventBeginPlay
  (Rendering|SceneCapture|ShowOnlyActorComponents (Variables|Default|GetSceneCaptureComponent2D) self true))

(fn ConstructionScript)