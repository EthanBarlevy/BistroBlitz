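; Holdable order for Bistro Blitz that shows a food order on its widget and reports itself as an order through the parent's object-information interface.
; CreateRandomOrder asks the UI_Order widget for an order, usually a chosen one and occasionally a randomly built one, then stores and returns it.
; It then calls CreateOrderServer, which has the widget build the stored order.
; CreateOrderMulti runs the same display logic but is not called here.
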(event Custom|CreateOrder%20Server
  (bind _asui_order (Utilities|Casting|CastToUI_Order (UserInterface|GetWidget (Variables|Default|GetWidget))))
  (Default|MakeIt _asui_order (Variables|Default|GetOrder)))

(event Custom|CreateOrder%20Multi
  (bind _asui_order (Utilities|Casting|CastToUI_Order (UserInterface|GetWidget (Variables|Default|GetWidget))))
  (Default|MakeIt _asui_order (Variables|Default|GetOrder)))

(event EventBeginPlay
  (|CallParentFunction) ; This node is disabled and will not be called.\nDrag off pins to build functionality.
)

(event Collision|EventActorBeginOverlap
  (params (OtherActor :type Actor%20Object%20Reference))
  (|CallParentFunction OtherActor) ; This node is disabled and will not be called.\nDrag off pins to build functionality.
)

(event EventTick
  (params (DeltaSeconds :type Float%20%28single-precision%29))
  (|CallParentFunction DeltaSeconds) ; This node is disabled and will not be called.\nDrag off pins to build functionality.
)

(fn ConstructionScript
  (|CallParentFunction))

(fn CreateRandomOrder
  (bind _asui_order (Utilities|Casting|CastToUI_Order (UserInterface|GetWidget (Variables|Default|GetWidget))))
  (if (== (Math|Random|RandomInteger 10) 0)
    (bind _order (Default|CreateRandomOrder _asui_order))
    (Variables|Default|SetOrder _order)
    (else
      (bind _order_2 (Default|ChooseOrder _asui_order))
      (Variables|Default|SetOrder _order_2)))
  (CallFunction|CreateOrderServer)
  (return (Variables|Default|GetOrder)))

(fn GetObjectInformation
  (bind (_canbecut _hasbeencut _canbecooked _hasbeencooked _isplate _ispan _isnothing _ismop _isorder _hasfood _objectname) (|CallParentFunction))
  (return _canbecut _hasbeencut _canbecooked _hasbeencooked _isplate _ispan _isnothing _ismop true _hasfood _objectname))