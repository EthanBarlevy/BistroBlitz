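; BP_Plate is the plate holdable in BistroBlitz, which stores the holdables added to it.
; AddItem appends to its Holdables array, from which GetFood gathers item names and GetMeshes reads static meshes, though GetMeshes returns inside its loop after the first entry.
; GetObjectInformation overrides the parent's result to flag IsPlate, report its HasFood variable and set ObjectName to None, passing other flags through.
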(event EventBeginPlay
  (|CallParentFunction) ; This node is disabled and will not be called.\nDrag off pins to build functionality.
)

(event Collision|EventActorBeginOverlap
  (params (OtherActor :type Actor%20Object%20Reference))
  (|CallParentFunction OtherActor) ; This node is disabled and will not be called.\nDrag off pins to build functionality.
)

(event EventTick
  (params (DeltaSeconds :type Float%20%28single-precision%29))
  (|CallParentFunction DeltaSeconds) ; This node is disabled and will not be called.\nDrag off pins to build functionality.
)

(fn ConstructionScript
  (|CallParentFunction))

(fn AddItem
  (params (Holdable :type BP%20Holdable%20Object%20Reference))
  (Utilities|Array|Add (Variables|Default|GetHoldables) Holdable)
  (Variables|Default|SetHoldables (Variables|Default|GetHoldables)))

(fn GetMeshes
  (Utilities|Array|Clear (Variables|Default|GetMeshes))
  (for _array_element (Variables|Default|GetHoldables)
    (Utilities|Array|Add (Variables|Default|GetMeshes) (Variables|/Script/Engine.StaticMeshComponent|GetStaticMesh (Variables|/Game/BistroBlitz/Blueprints/Holdables/BP_Holdable.BP_Holdable_C|GetStaticMesh _array_element)))
    (return (Variables|Default|GetMeshes))))

(fn GetFood
  (for _array_element (Variables|Default|GetHoldables)
    (Utilities|Array|Add (LocalVariables|GetNames) (Variables|/Game/BistroBlitz/Blueprints/Holdables/BP_Holdable.BP_Holdable_C|GetName _array_element)))
  (return (LocalVariables|GetNames)))

(fn GetObjectInformation
  (bind (_canbecut _hasbeencut _canbecooked _hasbeencooked _isplate _ispan _isnothing _ismop _isorder) (|CallParentFunction))
  (return _canbecut _hasbeencut _canbecooked _hasbeencooked true _ispan _isnothing _ismop _isorder (Variables|Default|GetHasFood) "None"))