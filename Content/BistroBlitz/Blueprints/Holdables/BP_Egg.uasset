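; Egg holdable for Bistro Blitz that changes its appearance between raw and cooked states.
; Overrides SetCooked to swap the static mesh between the whole egg and Egg4, lowering the Height offset when cooked, then calls the parent implementation.
; All other behavior is inherited, as the event graph holds only disabled stubs and construction just calls the parent.
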(event EventBeginPlay
  (|CallParentFunction) ; This node is disabled and will not be called.\nDrag off pins to build functionality.
)

(event Collision|EventActorBeginOverlap
  (params (OtherActor :type Actor%20Object%20Reference))
  (|CallParentFunction OtherActor) ; This node is disabled and will not be called.\nDrag off pins to build functionality.
)

(event EventTick
  (params (DeltaSeconds :type Float%20%28single-precision%29))
  (|CallParentFunction DeltaSeconds) ; This node is disabled and will not be called.\nDrag off pins to build functionality.
)

(fn ConstructionScript
  (|CallParentFunction))

(fn SetCooked
  (params (Cooked :type Boolean))
  (if Cooked
    (Components|StaticMesh|SetStaticMesh (Variables|Default|GetStaticMesh) "/Game/BistroBlitz/Models/egg4.egg4")
    (Variables|Default|SetHeight "0.000000,0.000000,2.000000")
    (else
      (Components|StaticMesh|SetStaticMesh (Variables|Default|GetStaticMesh) "/Game/BistroBlitz/Models/Egg_Whole.Egg_Whole")
      (Variables|Default|SetHeight "0.000000,0.000000,15.000000")))
  (|CallParentFunction Cooked))