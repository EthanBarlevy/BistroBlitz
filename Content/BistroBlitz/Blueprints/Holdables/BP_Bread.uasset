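; BP_Bread is the bread holdable in Bistro Blitz, with a whole and a cut state.
; It overrides SetCut to swap the static mesh between the bread and a slice, set a matching Height offset, then call the parent implementation.
; The event graph and construction script add no behavior of their own.
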(event EventBeginPlay
  (|CallParentFunction) ; This node is disabled and will not be called.\nDrag off pins to build functionality.
)

(event Collision|EventActorBeginOverlap
  (params (OtherActor :type Actor%20Object%20Reference))
  (|CallParentFunction OtherActor) ; This node is disabled and will not be called.\nDrag off pins to build functionality.
)

(event EventTick
  (params (DeltaSeconds :type Float%20%28single-precision%29))
  (|CallParentFunction DeltaSeconds) ; This node is disabled and will not be called.\nDrag off pins to build functionality.
)

(fn ConstructionScript
  (|CallParentFunction))

(fn SetCut
  (params (Cut :type Boolean))
  (if Cut
    (Components|StaticMesh|SetStaticMesh (Variables|Default|GetStaticMesh) "/Game/BistroBlitz/Models/BreadSlice12.BreadSlice12")
    (Variables|Default|SetHeight "0.000000,0.000000,3.500000")
    (else
      (Components|StaticMesh|SetStaticMesh (Variables|Default|GetStaticMesh) "/Game/BistroBlitz/Models/Bread.Bread")
      (Variables|Default|SetHeight "0.000000,0.000000,30.000000")))
  (|CallParentFunction Cut))