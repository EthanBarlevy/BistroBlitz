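; BP_Cheese is a holdable cheese ingredient in Bistro Blitz that can be whole or sliced.
; It overrides SetCut to swap the static mesh between Cheese and CheeseSlice, updating Height and Name to match before calling the parent implementation.
; The event graph holds only disabled default nodes, so all other behavior comes from the parent class.
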(event EventBeginPlay
  (|CallParentFunction) ; This node is disabled and will not be called.\nDrag off pins to build functionality.
)

(event Collision|EventActorBeginOverlap
  (params (OtherActor :type Actor%20Object%20Reference))
  (|CallParentFunction OtherActor) ; This node is disabled and will not be called.\nDrag off pins to build functionality.
)

(event EventTick
  (params (DeltaSeconds :type Float%20%28single-precision%29))
  (|CallParentFunction DeltaSeconds) ; This node is disabled and will not be called.\nDrag off pins to build functionality.
)

(fn ConstructionScript
  (|CallParentFunction))

(fn SetCut
  (params (Cut :type Boolean))
  (if Cut
    (Components|StaticMesh|SetStaticMesh (Variables|Default|GetStaticMesh) "/Game/BistroBlitz/Models/cheeseSlice.cheeseSlice")
    (Variables|Default|SetHeight "0.000000,0.000000,2.500000")
    (Variables|Default|SetName "Cheese-Sliced")
    (else
      (Components|StaticMesh|SetStaticMesh (Variables|Default|GetStaticMesh) "/Game/BistroBlitz/Models/cheese.cheese")
      (Variables|Default|SetHeight "0.000000,0.000000,15.000000")
      (Variables|Default|SetName "Cheese")))
  (|CallParentFunction Cut))