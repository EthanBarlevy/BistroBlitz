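; BP_Tomato is a holdable tomato ingredient in Bistro Blitz that can be either whole or sliced.
; It overrides SetCut, calling the parent and then swapping the static mesh, Height offset and display Name to match the cut state.
; The event graph holds only disabled stub events, and the construction script just calls the parent, so other behavior comes from the parent class.
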(event EventBeginPlay
  (|CallParentFunction) ; This node is disabled and will not be called.\nDrag off pins to build functionality.
)

(event Collision|EventActorBeginOverlap
  (params (OtherActor :type Actor%20Object%20Reference))
  (|CallParentFunction OtherActor) ; This node is disabled and will not be called.\nDrag off pins to build functionality.
)

(event EventTick
  (params (DeltaSeconds :type Float%20%28single-precision%29))
  (|CallParentFunction DeltaSeconds) ; This node is disabled and will not be called.\nDrag off pins to build functionality.
)

(fn ConstructionScript
  (|CallParentFunction))

(fn SetCut
  (params (Cut :type Boolean))
  (|CallParentFunction Cut)
  (if (Variables|Default|GetCut)
    (Components|StaticMesh|SetStaticMesh (Variables|Default|GetStaticMesh) "/Game/BistroBlitz/Models/tomatoSlice2.tomatoSlice2")
    (Variables|Default|SetHeight "0.000000,0.000000,2.300000")
    (Variables|Default|SetName "Tomato-Sliced")
    (else
      (Components|StaticMesh|SetStaticMesh (Variables|Default|GetStaticMesh) "/Game/BistroBlitz/Models/tomato.tomato")
      (Variables|Default|SetHeight "0.000000,0.000000,20.000000")
      (Variables|Default|SetName "Tomato"))))